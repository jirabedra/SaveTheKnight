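; Moving platform actor that travels back and forth along the spline of a referenced Track actor.
; Move starts the Mover timeline forward or in reverse based on Reverse, scaling play rate by Duration, and StopMoving halts it.
; Each update maps the timeline alpha to a distance along the spline and sets the world location without sweep.
; On finish, a FlipFlop toggles Reverse and restarts the timeline to alternate directions.
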(event `self.ReceiveBeginPlay`)

(event `Move`
  (`TimelineComponent.SetPlayRate` (`self.Mover`) (/ 1.0 (`self.Duration`)))
  (if (`self.Reverse`)
    (bind (_direction _alpha) (`Timeline|Mover` :!via `Reverse` :!label _label)
      (:`Update`
        (set `self.AlphaTrack` _alpha)
        (`self.K2_SetActorLocation` (`SplineComponent.GetLocationAtDistanceAlongSpline` (`/Game/Blueprints/SplineTracks/Track1.Spline` (`self.Track`)) (`KismetMathLibrary.Lerp` 0.0 (`SplineComponent.GetSplineLength` (`/Game/Blueprints/SplineTracks/Track1.Spline` (`self.Track`))) (`self.AlphaTrack`)) "World")))
      (:`Finished`
        (`/Engine/EditorBlueprintResources/StandardMacros.FlipFlop` ; Hace que ocurra secuencialmente ida y venida
          (:`A`
            (set `self.Reverse` true)
            (goto _label :!via `ReverseFromEnd`))
          (:`B`
            (set `self.Reverse` false)
            (goto _label :!via `PlayFromStart`)))))
    (else
      (goto _label))))

(event `StopMoving`
  (goto _label :!via `Stop`))

(fn `UserConstructionScript`)