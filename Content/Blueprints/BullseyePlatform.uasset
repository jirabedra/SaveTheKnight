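; BullseyePlatform is an actor that turns into a solid platform when a PrincessProjectile hits it.
; The construction script hides the Cube and disables its Collision component.
; On overlap with the projectile, it shows the Cube, enables query and physics collision, and prints a debug "Hello".
; It then hides the other cube and cylinder meshes and disables the Capsule collision, with no logic to revert.
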(event `self.ReceiveActorBeginOverlap`
  (params (OtherActor :type "Actor Object Reference"))
  (cast `/Game/Blueprints/PrincessProjectile` OtherActor)
  (`|ExecutionSequence`
    (:`then_0`
      (`SceneComponent.SetVisibility` (`self.Cube`) true false)
      (`PrimitiveComponent.SetCollisionEnabled` (`self.Collision`) "QueryAndPhysics")
      (`KismetSystemLibrary.PrintString` "Hello"))
    (:`then_1`
      (`SceneComponent.SetVisibility` (`self.Cube2`) false false)
      (`SceneComponent.SetVisibility` (`self.Cube3`) false false)
      (`SceneComponent.SetVisibility` (`self.Cylinder`) false false)
      (`PrimitiveComponent.SetCollisionEnabled` (`self.Capsule`) "NoCollision"))))

(fn `UserConstructionScript`
  (`SceneComponent.SetVisibility` (`self.Cube`) false false)
  (`PrimitiveComponent.SetCollisionEnabled` (`self.Collision`) "NoCollision"))