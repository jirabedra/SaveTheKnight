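; Pair of platforms that alternately appear and vanish on a fixed timer, so only one is solid at a time.
; BeginPlay hides the second cube and starts a looping timer that calls InvertPlatforms.
; That function sets each cube's visibility and collision opposite to the other from the IsCubeActive flag, then flips the flag.
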(event `self.ReceiveBeginPlay`
  (bind _cube1 (`self.Cube1`))
  (`SceneComponent.SetVisibility` _cube1 false false)
  (`PrimitiveComponent.SetCollisionEnabled` _cube1 "NoCollision")
  (`KismetSystemLibrary.K2_SetTimer` self "InvertPlatforms" 2.0 true))

(event `self.ReceiveActorBeginOverlap`
  (params (OtherActor :type "Actor Object Reference")))

(fn `InvertPlatforms`
  (bind _cube (`self.Cube`))
  (bind _iscubeactive (`self.IsCubeActive`))
  (bind _cube1 (`self.Cube1`))
  (`|ExecutionSequence`
    (:`then_0`
      ;[1 0.1719 0.1719] Invert cube status
      (`SceneComponent.SetVisibility` _cube (not _iscubeactive) false)
      (if (`self.IsCubeActive`)
        (`PrimitiveComponent.SetCollisionEnabled` _cube "NoCollision")
        (else
          (`PrimitiveComponent.SetCollisionEnabled` _cube "QueryAndPhysics"))))
    (:`then_1`
      ;[1 0.4746 0.1051] Invert cube 1 status
      (`SceneComponent.SetVisibility` _cube1 _iscubeactive false)
      (if (not (`self.IsCubeActive`))
        (`PrimitiveComponent.SetCollisionEnabled` _cube1 "NoCollision")
        (else
          (`PrimitiveComponent.SetCollisionEnabled` _cube1 "QueryAndPhysics")))
      (set `self.IsCubeActive` (not (`self.IsCubeActive`))))))

(fn `UserConstructionScript`)