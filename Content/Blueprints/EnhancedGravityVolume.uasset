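; A trigger volume that lets the third-person player character flip gravity while inside it.
; Entering enables the character's flip flags and icon, shows an interaction message widget for the player and opens a gate that lets NotifyActivation trigger the flip.
; When the player leaves, it removes the widget, hides the icon, closes the gate and flips gravity back if GravityScale is negative.
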(event `NotifyActivation`
  (`/Engine/EditorBlueprintResources/StandardMacros.Gate` true :!label _label
    (:`Exit`
      (bind _asthird_person_character (cast `/Game/ThirdPersonBP/Blueprints/ThirdPersonCharacter` (`GameplayStatics.GetPlayerCharacter` 0)))
      (`/Game/ThirdPersonBP/Blueprints/ThirdPersonCharacter.NotifyFlipGravity` _asthird_person_character))))

(event `self.ReceiveActorBeginOverlap`
  (params (OtherActor :type "Actor Object Reference"))
  (bind _asthird_person_character (cast `/Game/ThirdPersonBP/Blueprints/ThirdPersonCharacter` OtherActor))
  (set `/Game/ThirdPersonBP/Blueprints/ThirdPersonCharacter.ShowGravityIcon` true _asthird_person_character)
  (set `/Game/ThirdPersonBP/Blueprints/ThirdPersonCharacter.GravityFlipEnabled` true _asthird_person_character)
  (set `/Game/ThirdPersonBP/Blueprints/ThirdPersonCharacter.CanFlip` true _asthird_person_character)
  (if (`self.ActorHasTag` OtherActor "Player")
    (bind _returnvalue (`|CreateWidget` "/Game/UI/Widgets/GravityInteractionMessage.GravityInteractionMessage_C"))
    (`UserWidget.AddToViewport` _returnvalue 9)
    (goto _label :!via `Open`)))

(event `self.ReceiveActorEndOverlap`
  (params (OtherActor :type "Actor Object Reference"))
  (bind _returnvalue (`GameplayStatics.GetPlayerCharacter` 0))
  (if (`self.ActorHasTag` OtherActor "Player")
    (`Widget.RemoveFromParent` (stale `self.ReceiveActorBeginOverlap` _returnvalue))
    (`/Engine/EditorBlueprintResources/StandardMacros.IsValid` _returnvalue
      (:`Is Valid`
        (if (< (`CharacterMovementComponent.GravityScale` (`Character.CharacterMovement` _returnvalue)) 0.0)
          (bind _asthird_person_character (cast `/Game/ThirdPersonBP/Blueprints/ThirdPersonCharacter` _returnvalue))
          (set `/Game/ThirdPersonBP/Blueprints/ThirdPersonCharacter.ShowGravityIcon` false _asthird_person_character)
          (`/Game/ThirdPersonBP/Blueprints/ThirdPersonCharacter.NotifyFlipGravity` _asthird_person_character)
          (goto _label :!via `Close`)
          (else
            (bind _asthird_person_character_2 (cast `/Game/ThirdPersonBP/Blueprints/ThirdPersonCharacter` _returnvalue))
            (set `/Game/ThirdPersonBP/Blueprints/ThirdPersonCharacter.ShowGravityIcon` false _asthird_person_character_2)
            (goto _label :!via `Close`)))))))

(fn `UserConstructionScript`)