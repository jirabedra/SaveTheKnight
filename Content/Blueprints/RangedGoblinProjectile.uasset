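; Projectile actor for the ranged goblin that damages the player on impact.
; On hit, it checks that the actor is Damageable and tagged Player, sends a small fixed DealDamage message, prints a debug string and destroys itself.
; The DealDamage event casts the target to Princess and calls ReceiveDamage, passing itself as the Damaging causer.
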(event `self.ReceiveBeginPlay`)

(event `self.ReceiveActorBeginOverlap`
  (params (OtherActor :type "Actor Object Reference")))

(event `self.ReceiveHit`
  (params (MyComp :type "PrimitiveComponent Object Reference") (Other :type "Actor Object Reference") (OtherComp :type "PrimitiveComponent Object Reference") (bSelfMoved :type Boolean) (HitLocation :type "Vector Structure") (HitNormal :type "Vector Structure") (NormalImpulse :type "Vector Structure") (Hit :type "HitResult Structure (by ref)"))
  (bind (_bblockinghit _binitialoverlap _time _distance _location _impactpoint _normal _impactnormal _physmat _hitactor) (`GameplayStatics.BreakHitResult` Hit))
  (bind _asdamageable (cast `/Game/Blueprints/Interfaces/Damageable` _hitactor))
  (if (`self.ActorHasTag` _hitactor "Player")
    (`KismetSystemLibrary.PrintString` "hit")
    (message `/Game/Blueprints/Interfaces/Damaging.DealDamage` self 0.04 _asdamageable)
    (`self.K2_DestroyActor`)))

(event `/Game/Blueprints/Interfaces/Damaging.DealDamage`
  (params (DamageAmount :type "Float (single-precision)") (Target :type "/Game/Blueprints/Interfaces/Damageable Interface"))
  (bind _asprincess (cast `/Game/ThirdPersonBP/Blueprints/Princess` Target))
  (bind _asdamaging (cast `/Game/Blueprints/Interfaces/Damaging` self))
  (`/Game/ThirdPersonBP/Blueprints/Princess.ReceiveDamage` _asprincess DamageAmount _asdamaging))

(fn `UserConstructionScript`)