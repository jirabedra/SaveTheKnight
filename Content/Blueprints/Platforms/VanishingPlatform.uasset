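; Platform that crumbles away after a Player-tagged actor overlaps it, then restores itself.
; After a short delay, a Sequence with parallel Delays hides and disables collision on five meshes in staggered order, starting with the fifth.
; The Box collision switches off with that first mesh.
; A longer Delay on the same Sequence later restores all meshes and the Box at once.
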(event `self.ReceiveActorBeginOverlap`
  (params (OtherActor :type "Actor Object Reference"))
  (bind _staticmesh (`self.StaticMesh`))
  (bind _staticmesh3 (`self.StaticMesh3`))
  (bind _staticmesh4 (`self.StaticMesh4`))
  (bind _staticmesh1 (`self.StaticMesh1`))
  (bind _staticmesh2 (`self.StaticMesh2`))
  (if (`self.ActorHasTag` OtherActor "Player")
    (`KismetSystemLibrary.Delay` 1.0)
    (`|ExecutionSequence`
      (:`then_0`
        ;[1 0.1719 0.1719] Vanish mesh 1
        (`KismetSystemLibrary.Delay` 0.25)
        (`SceneComponent.SetVisibility` _staticmesh false false)
        (`PrimitiveComponent.SetCollisionEnabled` _staticmesh "NoCollision"))
      (:`then_1`
        ;[1 0.4746 0.1051] Vanish mesh 2
        (`KismetSystemLibrary.Delay` 0.5)
        (`SceneComponent.SetVisibility` _staticmesh1 false false)
        (`PrimitiveComponent.SetCollisionEnabled` _staticmesh1 "NoCollision"))
      (:`then_2`
        ;[1 0.9542 0.165] Vanish mesh 3
        (`KismetSystemLibrary.Delay` 0.75)
        (`SceneComponent.SetVisibility` _staticmesh2 false false)
        (`PrimitiveComponent.SetCollisionEnabled` _staticmesh2 "NoCollision"))
      (:`then_3`
        ;[0.3498 1 0.3198] Vanish mesh 4
        (`KismetSystemLibrary.Delay` 1.0)
        (`SceneComponent.SetVisibility` _staticmesh3 false false)
        (`PrimitiveComponent.SetCollisionEnabled` _staticmesh3 "NoCollision"))
      (:`then_4`
        ;[0.2915 0.4264 1] Vanish mesh 5
        (`SceneComponent.SetVisibility` _staticmesh4 false false)
        (`PrimitiveComponent.SetCollisionEnabled` _staticmesh4 "NoCollision")
        (`PrimitiveComponent.SetCollisionEnabled` (`self.Box`) "NoCollision"))
      (:`then_5`
        (`KismetSystemLibrary.Delay` 3.5)
        (`|ExecutionSequence`
          (:`then_0`
            ;[1 0.1719 0.1719] Reappear mesh 1
            (`SceneComponent.SetVisibility` _staticmesh true false)
            (`PrimitiveComponent.SetCollisionEnabled` _staticmesh "QueryAndPhysics")
            (`PrimitiveComponent.SetCollisionEnabled` (`self.Box`) "QueryAndPhysics"))
          (:`then_1`
            ;[1 0.4746 0.1051] Reappear mesh 2
            (`SceneComponent.SetVisibility` _staticmesh1 true false)
            (`PrimitiveComponent.SetCollisionEnabled` _staticmesh1 "QueryAndPhysics"))
          (:`then_2`
            ;[1 0.9542 0.165] Reappear mesh 3
            (`SceneComponent.SetVisibility` _staticmesh2 true false)
            (`PrimitiveComponent.SetCollisionEnabled` _staticmesh2 "QueryAndPhysics"))
          (:`then_3`
            ;[0.3498 1 0.3198] Reappear mesh 4
            (`SceneComponent.SetVisibility` _staticmesh3 true false)
            (`PrimitiveComponent.SetCollisionEnabled` _staticmesh3 "QueryAndPhysics"))
          (:`then_4`
            ;[0.2915 0.4264 1] Reappear mesh 5
            (`SceneComponent.SetVisibility` _staticmesh4 true false)
            (`PrimitiveComponent.SetCollisionEnabled` _staticmesh4 "QueryAndPhysics")))))))

(fn `UserConstructionScript`)