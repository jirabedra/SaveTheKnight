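; FloatingBullseye is a target actor that reacts when hit by a PrincessProjectile.
; On overlap it destroys the projectile, hides its cylinder mesh and turns off collision on its capsule and box, so it stays in the level but is inert.
; It then plays the Bullseye sound in 2D at the SFX volume read from the GameData game instance.
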(event `self.ReceiveBeginPlay`)

(event `self.ReceiveActorBeginOverlap`
  (params (OtherActor :type "Actor Object Reference"))
  (bind _asprincess_projectile (cast `/Game/Blueprints/PrincessProjectile` OtherActor))
  (`self.K2_DestroyActor` _asprincess_projectile)
  (`SceneComponent.SetVisibility` (`self.Cylinder`) false false)
  (`PrimitiveComponent.SetCollisionEnabled` (`self.Capsule`) "NoCollision")
  (`PrimitiveComponent.SetCollisionEnabled` (`self.Box`) "NoCollision")
  (`GameplayStatics.PlaySound2D` "/Game/Sound/SFX/Bullseye.Bullseye" (`/Game/GameData.SFXVolumeValue` (cast `/Game/GameData` (`GameplayStatics.GetGameInstance`) :!pure true)) 1.0 0.0 null null))

(fn `UserConstructionScript`)