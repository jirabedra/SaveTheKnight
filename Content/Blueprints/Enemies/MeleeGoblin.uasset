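; Melee goblin enemy that damages the player Princess at close range and cackles at random while alive.
; MeleeAttack finds Princess actors overlapping the capsule, plays the attack montage on those tagged Player, and sends damage through the Damageable and Damaging interfaces.
; Tick refreshes the health bar widget from doubled Health and runs a random countdown that occasionally plays one of two laughs at the game instance's SFX volume.
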(event `self.ReceiveBeginPlay`
  (`parent.ReceiveBeginPlay`)
  (bind _output_get (set `self.TimeBetweenLaughs` (`KismetMathLibrary.RandomFloatInRange` 7.0 15.0)))
  (set `self.TimeToLaughRemaining` _output_get)
  (set `self.HealthBarRef` (cast `/Game/UI/3DWidgets/HealthBar` (`WidgetComponent.GetUserWidgetObject` (`self.Widget`)) :!pure true)))

(event `self.ReceiveTick`
  (params (DeltaSeconds :type "Float (single-precision)"))
  (bind _returnvalue (`self.K2_GetActorLocation`))
  (bind _sfxvolumevalue (`/Game/GameData.SFXVolumeValue` (cast `/Game/GameData` (`GameplayStatics.GetGameInstance`) :!pure true)))
  (`parent.ReceiveTick` DeltaSeconds)
  (`ProgressBar.SetPercent` (`/Game/UI/3DWidgets/HealthBar.HealthBar` (`self.HealthBarRef`)) (* 2 (`self.Health`)))
  ;[1 1 1] Play sound randomly
  (set `self.TimeToLaughRemaining` (- (`self.TimeToLaughRemaining`) DeltaSeconds))
  (if (<= (`self.TimeToLaughRemaining`) 0.0)
    (set `self.TimeToLaughRemaining` (`KismetMathLibrary.RandomFloatInRange` 7.0 15.0))
    (if (< (`KismetMathLibrary.RandomFloatInRange` 0.0 1.0) 0.25)
      (if (< (`KismetMathLibrary.RandomFloatInRange` 0.0 2.0) 1.0)
        (`GameplayStatics.PlaySoundAtLocation` "/Game/Sound/SFX/Goblin/GoblinLaugh.GoblinLaugh" _returnvalue (struct) _sfxvolumevalue 1.0 0.0 null null null)
        (else
          (`GameplayStatics.PlaySoundAtLocation` "/Game/Sound/SFX/Goblin/GoblinLaugh2.GoblinLaugh2" _returnvalue (struct) _sfxvolumevalue 1.0 0.0 null null null))))))

(event `/Game/Blueprints/Interfaces/MeleeEnemy.MeleeAttack`
  (`self.NotifyMeleeAttack`)
  (for _array_element (`PrimitiveComponent.GetOverlappingActors` (`self.Capsule`) "/Game/ThirdPersonBP/Blueprints/Princess.Princess_C")
    (bind _asdamageable (cast `/Game/Blueprints/Interfaces/Damageable` _array_element))
    (if (`self.ActorHasTag` _array_element "Player")
      (`|PlayMontage` (`self.Mesh`) "/Game/STKAssets/Goblins/MeleeGoblin/Attack_Montage.Attack_Montage"
        (:`then`
          (message `/Game/Blueprints/Interfaces/Damaging.DealDamage` self 0.07 _asdamageable)
          (`KismetSystemLibrary.Delay` 2.0))))))

(event `/Game/Blueprints/Interfaces/Damaging.DealDamage`
  (params (DamageAmount :type "Float (single-precision)") (Target :type "/Game/Blueprints/Interfaces/Damageable Interface"))
  (bind _asprincess (cast `/Game/ThirdPersonBP/Blueprints/Princess` Target))
  (bind _asdamaging (cast `/Game/Blueprints/Interfaces/Damaging` self))
  (`/Game/ThirdPersonBP/Blueprints/Princess.ReceiveDamage` _asprincess DamageAmount _asdamaging))

(fn `UserConstructionScript`
  (`parent.UserConstructionScript`))