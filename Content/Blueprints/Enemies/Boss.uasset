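; Dragon boss enemy that owns its health, creates a boss HUD and updates its health bar every tick.
; Notify events run five attacks (pillar cleave, frontal cone, tail swipe, rotating circular breath, triple fire aura) as delayed spawn-and-destroy collision actors with sounds and flags.
; Pillar cleave and fire aura show on-screen widgets; cleave damages the Princess when no pillars remain.
; A timeline yaws the boss during circular breath, dragging the breath collision along.
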(event `self.ReceiveBeginPlay`
  (`parent.ReceiveBeginPlay`)
  (bind _output_get (set `self.MaxHealth` 60.0))
  (set `self.Health` _output_get)
  (bind _returnvalue (`|CreateWidget` "/Game/UI/BossHUD.BossHUD_C"))
  (bind _output_get_2 (set `self.HUD` _returnvalue))
  (`UserWidget.AddToViewport` _output_get_2 0)
  (`KismetSystemLibrary.Delay` 8.0))

(event `self.ReceiveTick`
  (params (DeltaSeconds :type "Float (single-precision)"))
  (`parent.ReceiveTick` DeltaSeconds)
  (`/Game/UI/BossHUD.UpdateHealthBar` (`self.HUD`) (`self.Health`) (`self.MaxHealth`)))

(event `NotifyPillarCleave`
  ;[1 0.4453 0.7623] PILLAR CLEAVE SUMMON SOLO F2
  (`GameplayStatics.PlayWorldCameraShake` "/Game/STKAssets/BossRoom/BP_CleaveShake.BP_CleaveShake_C" (0.0 0.0 0.0) 0.0 500000.0 5.0)
  (bind _returnvalue (`|CreateWidget` "/Game/UI/3DWidgets/BossPillarWidget.BossPillarWidget_C"))
  (`UserWidget.AddToViewport` _returnvalue 9)
  (`KismetSystemLibrary.Delay` 4.0)
  (`Widget.RemoveFromParent` _returnvalue)
  (set `self.bFlaggedToSummonPillarCleave` true)
  (`KismetSystemLibrary.Delay` 0.2)
  (bind _returnvalue_2 (`|SpawnActorFromClass` "/Game/Blueprints/Enemies/BossSkillCollision/BP_PillarCleave.BP_PillarCleave_C" (`SceneComponent.K2_GetComponentToWorld` (`self.RaycastingMesh`)) "Undefined" "OverrideRootScale" self null))
  (set `/Game/Blueprints/Enemies/BossSkillCollision/BP_PillarCleave.WallRef` (`self.WallRef`) _returnvalue_2)
  (set `self.bFlaggedToSummonPillarCleave` false)
  (`KismetSystemLibrary.Delay` 2.0)
  (`self.PlayBuildingSound`)
  ;;[1 1 1] Acá podría ir otro camera shake
  (`|ExecutionSequence`
    (:`then_0`
      (if (== (`KismetArrayLibrary.Array_Length` (`self.Pillars`)) 0)
        (`/Game/Blueprints/Interfaces/Damageable.TakeDamage` (cast `/Game/ThirdPersonBP/Blueprints/Princess` (`GameplayStatics.GetPlayerCharacter` 0) :!pure true) 1.0)))
    (:`then_1`
      (`self.K2_DestroyActor` _returnvalue_2))))

(event `NotifyFrontalCone`
  ;[0.1188 1 0.1619] FRONTAL CONE SUMMON F1 F2
  (set `self.bFlaggedToSummonFrontalCone` true)
  (`KismetSystemLibrary.Delay` 1.5)
  (bind _returnvalue (`|SpawnActorFromClass` "/Game/Blueprints/Enemies/BossSkillCollision/BP_FrontalConeCollision.BP_FrontalConeCollision_C" (`KismetMathLibrary.MakeTransform` (`SceneComponent.K2_GetComponentLocation` (`self.SkillEmittingMesh`)) (`self.K2_GetActorRotation` self) (15.0 15.0 15.0)) "Undefined" "OverrideRootScale" self null))
  (`KismetSystemLibrary.Delay` 0.2)
  (set `self.bFlaggedToSummonFrontalCone` false)
  (`KismetSystemLibrary.Delay` 2.8)
  (`self.K2_DestroyActor` _returnvalue))

(event `NotifyTailSwipe`
  ;[1 0.8574 0.1197] TAIL SWIPE SUMMON F1F2
  (set `self.bFlaggedToSummonTailSwipe` true)
  (`KismetSystemLibrary.Delay` 1.0)
  (`self.PlayGrowlSound`)
  (bind _returnvalue (`|SpawnActorFromClass` "/Game/Blueprints/Enemies/BossSkillCollision/BP_TailSwipeCollision.BP_TailSwipeCollision_C" (`KismetMathLibrary.MakeTransform` (`KismetMathLibrary.MakeVector` (.x (`self.K2_GetActorLocation` self)) (.y (`self.K2_GetActorLocation` self))) (struct) (30.0 30.0 30.0)) "Undefined" "OverrideRootScale" null null))
  (`KismetSystemLibrary.Delay` 0.2)
  (set `self.bFlaggedToSummonTailSwipe` false)
  (`KismetSystemLibrary.Delay` 2.8)
  (`self.K2_DestroyActor` _returnvalue))

(event `NotifyCircularBreath`
  ;[0.4886 0.5173 1] CIRCULAR BREATH SUMMON F2
  (`GameplayStatics.PlaySoundAtLocation` "/Game/Sound/SFX/Dragon/DragonFire.DragonFire" (`self.K2_GetActorLocation`) (struct) (`/Game/GameData.SFXVolumeValue` (cast `/Game/GameData` (`GameplayStatics.GetGameInstance`) :!pure true)) 1.0 0.0 null null null)
  (bind _returnvalue (`|SpawnActorFromClass` "/Game/Blueprints/Enemies/BossSkillCollision/BP_CircularBreathCollision.BP_CircularBreathCollision_C" (`KismetMathLibrary.MakeTransform` (`KismetMathLibrary.MakeVector` (.x (`SceneComponent.K2_GetComponentLocation` (`self.SkillEmittingMesh`))) (.y (`SceneComponent.K2_GetComponentLocation` (`self.SkillEmittingMesh`))) (.z (`SceneComponent.K2_GetComponentLocation` (`self.SkillEmittingMesh`)))) (`KismetMathLibrary.MakeRotator` (.roll (`self.K2_GetActorRotation` self)) (.pitch (`self.K2_GetActorRotation` self)) (+ (.yaw (`self.K2_GetActorRotation` self)) 0.0)) (15.0 15.0 15.0)) "Undefined" "OverrideRootScale" self null))
  (bind (_direction _newtrack_0) (`Timeline|YawRotation` :!via `PlayFromStart`)
    (:`Update`
      (`self.K2_SetActorRelativeRotation` (`KismetMathLibrary.MakeRotator` 0.0 0.0 _newtrack_0))
      (`self.K2_SetActorLocation` _returnvalue (`SceneComponent.K2_GetComponentLocation` (`self.SkillEmittingMesh`)) false false)
      (`self.K2_SetActorRelativeRotation` _returnvalue (`self.K2_GetActorRotation` self) false false))
    (:`Finished`
      (`self.K2_DestroyActor` _returnvalue))))

(event `NotifyFireAura`
  ;[1 1 1] FIRE AURA SUMMON F1F2
  (bind _returnvalue (`|CreateWidget` "/Game/UI/3DWidgets/BossAuraWidget.BossAuraWidget_C"))
  (`UserWidget.AddToViewport` _returnvalue 9)
  (`KismetSystemLibrary.Delay` 2.0)
  (`self.SingleFireAura`)
  (`KismetSystemLibrary.Delay` 1.5)
  (`self.SingleFireAura`)
  (`KismetSystemLibrary.Delay` 1.5)
  (`self.SingleFireAura`)
  (`Widget.RemoveFromParent` _returnvalue))

(event `SingleFireAura`
  ;[1 1 1] FIRE AURA SUMMON F1F2
  (`self.PlayGrowlSound`)
  (bind _returnvalue (`|SpawnActorFromClass` "/Game/Blueprints/Enemies/BossSkillCollision/BP_FireAura.BP_FireAura_C" (`KismetMathLibrary.MakeTransform` (`KismetMathLibrary.MakeVector` (.x (.location (`self.GetTransform` self))) (.y (.location (`self.GetTransform` self))) 100.0)) "Undefined" "OverrideRootScale" self null))
  (`KismetSystemLibrary.Delay` 1.0)
  (`self.K2_DestroyActor` _returnvalue))

(fn `PlayAttackSound`
  (`GameplayStatics.PlaySoundAtLocation` "/Game/Sound/SFX/Dragon/DragonAttack.DragonAttack" (`self.K2_GetActorLocation`) (struct) (`/Game/GameData.SFXVolumeValue` (cast `/Game/GameData` (`GameplayStatics.GetGameInstance`) :!pure true)) 1.0 0.0 null null null))

(fn `PlayBuildingSound`
  (`GameplayStatics.PlaySoundAtLocation` "/Game/Sound/SFX/Dragon/BuildingBreaking.BuildingBreaking" (`self.K2_GetActorLocation`) (struct) (`/Game/GameData.SFXVolumeValue` (cast `/Game/GameData` (`GameplayStatics.GetGameInstance`) :!pure true)) 1.0 0.0 null null null))

(fn `PlayGrowlSound`
  (`GameplayStatics.PlaySoundAtLocation` "/Game/Sound/SFX/Dragon/DragonGrowl.DragonGrowl" (`self.K2_GetActorLocation`) (struct) (`/Game/GameData.SFXVolumeValue` (cast `/Game/GameData` (`GameplayStatics.GetGameInstance`) :!pure true)) 1.0 0.0 null null null))

(fn `UserConstructionScript`
  (`parent.UserConstructionScript`))