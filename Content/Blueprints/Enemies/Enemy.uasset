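; Enemy actor with a health pool that can be hurt by princess projectiles and death planes.
; ReceiveDamage filters the damage causer by casting to those two classes and forwards accepted hits to the TakeDamage event.
; TakeDamage destroys the actor when health runs out; otherwise it subtracts the damage and grants brief immunity through a Delay, ignoring further hits until it ends.
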(event `self.TakeDamage`
  (params (DamageAmount :type "Float (single-precision)"))
  (if (`self.Immune`)
    _
    (elif (<= (- (`self.Health`) DamageAmount) 0.0)
      (set `self.Health` 0.0)
      (`self.K2_DestroyActor`)
      (else
        (set `self.Health` (- (`self.Health`) DamageAmount))
        (set `self.Immune` true)
        (`KismetSystemLibrary.Delay` 1.0)
        (set `self.Immune` false)))))

(fn `ReceiveDamage`
  (params (DamageAmount :type "Float (double-precision)") (DamageCauser :type "/Game/Blueprints/Interfaces/Damaging Interface"))
  (cast `/Game/Blueprints/PrincessProjectile` DamageCauser
    (:`then`
      (`self.TakeDamage` DamageAmount))
    (:`CastFailed`
      (cast `/Game/Blueprints/Obstacles/Terrain/DeathPlane` DamageCauser)
      (`self.TakeDamage` DamageAmount))))

(fn `UserConstructionScript`)