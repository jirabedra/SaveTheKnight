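; AI controller for the ranged goblin enemy that runs its behavior tree and feeds it game state through the blackboard.
; On BeginPlay it sets up the blackboard with the player character as target, then starts the tree.
; Perception updates on the Princess set the line-of-sight flag.
; Tick polls the controlled Enemy's health, re-invoking UseBlackboard and flagging it dead whenever health equals zero.
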(event `self.ReceiveBeginPlay`
  (bind _blackboardcomponent (`self.UseBlackboard` "/Game/Blueprints/Enemies/SimpleAI/RangedGoblinBB.RangedGoblinBB"))
  (`BlackboardComponent.SetValueAsObject` _blackboardcomponent (`self.Player`) (`GameplayStatics.GetPlayerCharacter` 0))
  (`self.RunBehaviorTree` "/Game/Blueprints/Enemies/SimpleAI/RangedGoblinBT.RangedGoblinBT"))

(event `self.AIPerception.OnTargetPerceptionUpdated`
  (params (Actor :type "Actor Object Reference") (Stimulus :type "AIStimulus Structure"))
  (cast `/Game/ThirdPersonBP/Blueprints/Princess` Actor)
  (`BlackboardComponent.SetValueAsBool` (`AIBlueprintHelperLibrary.GetBlackboard` null) "HasLineOfSight" (`.bSuccessfullySensed` (break `AIStimulus` Stimulus))))

(event `self.ReceiveTick`
  (params (DeltaSeconds :type "Float (single-precision)"))
  (bind _asenemy (cast `/Game/Blueprints/Enemies/Enemy` (`self.K2_GetPawn`)))
  (if (== (`/Game/Blueprints/Enemies/Enemy.Health` _asenemy) 0.0)
    (bind _blackboardcomponent (`self.UseBlackboard` "/Game/Blueprints/Enemies/SimpleAI/RangedGoblinBB.RangedGoblinBB"))
    (`BlackboardComponent.SetValueAsBool` _blackboardcomponent "Dead" true)))

(fn `UserConstructionScript`)