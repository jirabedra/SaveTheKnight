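; RangedGoblin is an enemy Blueprint whose main logic is a Shoot function that fires a RangedGoblinProjectile.
; The spawn point is the Sphere's location plus a gun offset rotated by the mesh, and the direction is the mesh's forward vector rotated by a shoot offset.
; An IsShooting flag brackets the spawn, the PlayerLocation input goes unused, and the event graph holds only disabled default events.
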(fn `Shoot`
  (params (PlayerLocation :type "Transform Structure"))
  (bind _returnvalue (`SceneComponent.K2_GetComponentRotation` (`self.Mesh`)))
  (set `self.IsShooting` true)
  (`|SpawnActorFromClass` "/Game/Blueprints/RangedGoblinProjectile.RangedGoblinProjectile_C" (`KismetMathLibrary.MakeTransform` (+ (`SceneComponent.K2_GetComponentLocation` (`self.Sphere`)) (`KismetMathLibrary.GreaterGreater_VectorRotator` (`self.GunOffset`) _returnvalue)) (`KismetMathLibrary.Conv_VectorToRotator` (`KismetMathLibrary.Quat_RotateVector` (`KismetMathLibrary.Conv_VectorToQuaternion` (`self.ShootOffset`)) (`KismetMathLibrary.Conv_RotatorToVector` _returnvalue)))) "Undefined" "OverrideRootScale" null null)
  (set `self.IsShooting` false))

(fn `UserConstructionScript`
  (`parent.UserConstructionScript`))