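; Boss skill actor for the pillar cleave attack, resolved by a single line trace shortly after spawning.
; After a brief delay it traces the Camera channel along its owner's forward direction, ignoring the owner and WallRef.
; A hit Pillar is notified and a hit Princess takes damage; any other hit or a miss damages the player character instead.
; The trace leaves persistent debug lines and prints the hit actor's name.
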(event `self.ReceiveBeginPlay`
  (bind _returnvalue (`self.GetOwner`))
  (bind _returnvalue_2 (`self.K2_GetActorLocation` self))
  (`KismetSystemLibrary.Delay` 0.2)
  (bind (_outhit _returnvalue_3) (`KismetSystemLibrary.LineTraceSingle` _returnvalue_2 (+ _returnvalue_2 (* (`KismetMathLibrary.GetForwardVector` (`self.K2_GetActorRotation` _returnvalue)) 3000.0)) "TraceTypeQuery2" false (`|MakeArray` _returnvalue (`self.WallRef`) :!type "Actor Object Reference") "Persistent" true (struct :`G` 0.017571 :`B` 1.0 :`A` 1.0) (struct :`R` 1.0 :`G` 0.077081 :`B` 0.896316 :`A` 1.0)))
  (if _returnvalue_3
    (bind (_bblockinghit _binitialoverlap _time _distance _location _impactpoint _normal _impactnormal _physmat _hitactor) (`GameplayStatics.BreakHitResult` _outhit))
    (`KismetSystemLibrary.PrintString` (`KismetSystemLibrary.GetDisplayName` _hitactor))
    ;[0.4598 0.6442 1] Case pillar has been hit
    (bind _aspillar (cast `/Game/STKAssets/BossRoom/Pillar` _hitactor)
      (:`then`
        (`/Game/STKAssets/BossRoom/Pillar.NotifyBossCleaveHit` _aspillar))
      (:`CastFailed`
        ;[1 0.07812 0.07812] Case princess has been hit
        (bind _asprincess (cast `/Game/ThirdPersonBP/Blueprints/Princess` _hitactor)
          (:`then`
            (bind _asdamageable (cast `/Game/Blueprints/Interfaces/Damageable` _asprincess))
            (`/Game/Blueprints/Interfaces/Damageable.TakeDamage` _asdamageable 1.0))
          (:`CastFailed`
            ;[1 0 0] Case nothing relevant has been hit
            (bind _asdamageable_2 (cast `/Game/Blueprints/Interfaces/Damageable` (`GameplayStatics.GetPlayerCharacter` 0) :!label _label))
            (`/Game/Blueprints/Interfaces/Damageable.TakeDamage` _asdamageable_2 1.0)))))
    (else
      (goto _label))))

(fn `UserConstructionScript`)