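; BP_FireAura is a boss skill actor that shows a growing fire aura and damages the Princess.
; On BeginPlay, a Scale timeline drives the uniform scale of the NS effect.
; Each timeline update also casts 360 one-degree-spaced line traces around the owner's rotation on the Camera channel, ignoring the owner and WallRef.
; Trace length is fixed, independent of scale, and each Princess hit applies a small Damageable hit.
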(event `self.ReceiveBeginPlay`
  (bind _returnvalue (`self.GetOwner`))
  (bind _returnvalue_2 (`self.K2_GetActorLocation` self))
  (bind (_direction _newtrack_0) (`Timeline|Scale` :!via `PlayFromStart`)
    (:`Update`
      (`SceneComponent.SetRelativeScale3D` (`self.NS`) (`KismetMathLibrary.MakeVector` _newtrack_0 _newtrack_0 _newtrack_0))
      (for _index (range 360)
        (bind (_outhit _returnvalue_3) (`KismetSystemLibrary.LineTraceSingle` _returnvalue_2 (+ _returnvalue_2 (* (`KismetMathLibrary.GetForwardVector` (`KismetMathLibrary.MakeRotator` (.roll (`self.K2_GetActorRotation` _returnvalue)) (.pitch (`self.K2_GetActorRotation` _returnvalue)) (+ (`KismetMathLibrary.Conv_IntToDouble` _index) (.yaw (`self.K2_GetActorRotation` _returnvalue))))) 5000.0)) "TraceTypeQuery2" true (`|MakeArray` _returnvalue (`self.WallRef`) :!type "Actor Object Reference") "None" true (struct :`R` 0.989583 :`G` 1.0 :`B` 0.979167 :`A` 1.0) (struct :`R` 1.0 :`G` 0.077081 :`B` 0.896316 :`A` 1.0) 0.2))
        (if _returnvalue_3
          (bind (_bblockinghit _binitialoverlap _time _distance _location _impactpoint _normal _impactnormal _physmat _hitactor) (`GameplayStatics.BreakHitResult` _outhit))
          ;[1 0.07812 0.07812] Case princess has been hit
          (bind _asprincess (cast `/Game/ThirdPersonBP/Blueprints/Princess` _hitactor))
          (bind _asdamageable (cast `/Game/Blueprints/Interfaces/Damageable` _asprincess))
          (`/Game/Blueprints/Interfaces/Damageable.TakeDamage` _asdamageable 0.1)
          (`KismetSystemLibrary.PrintString` (`KismetSystemLibrary.GetDisplayName` _hitactor)))))))

(fn `UserConstructionScript`)