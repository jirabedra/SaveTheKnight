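; Basilisk enemy Blueprint that deals melee damage to the player's Princess.
; MeleeAttack calls NotifyMeleeAttack, then scans capsule overlaps for Damageable, Player-tagged Princess actors and sends a small fixed DealDamage message, followed by a Delay that gates nothing.
; DealDamage casts the target to Princess and itself to Damaging, then calls ReceiveDamage with the Basilisk as causer.
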(event `/Game/Blueprints/Interfaces/MeleeEnemy.MeleeAttack`
  (`self.NotifyMeleeAttack`)
  (for _array_element (`PrimitiveComponent.GetOverlappingActors` (`self.Capsule`) "/Game/ThirdPersonBP/Blueprints/Princess.Princess_C")
    (bind _asdamageable (cast `/Game/Blueprints/Interfaces/Damageable` _array_element))
    (if (`self.ActorHasTag` _array_element "Player")
      (message `/Game/Blueprints/Interfaces/Damaging.DealDamage` self 0.07 _asdamageable)
      (`KismetSystemLibrary.Delay` 2.0))))

(event `/Game/Blueprints/Interfaces/Damaging.DealDamage`
  (params (DamageAmount :type "Float (single-precision)") (Target :type "/Game/Blueprints/Interfaces/Damageable Interface"))
  (bind _asprincess (cast `/Game/ThirdPersonBP/Blueprints/Princess` Target))
  (bind _asdamaging (cast `/Game/Blueprints/Interfaces/Damaging` self))
  (`/Game/ThirdPersonBP/Blueprints/Princess.ReceiveDamage` _asprincess DamageAmount _asdamaging))

(fn `UserConstructionScript`
  (`parent.UserConstructionScript`))