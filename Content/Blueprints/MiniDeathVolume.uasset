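; MiniDeathVolume is a volume that triggers an emergency flip on the player character.
; When an actor tagged Player begins overlapping it, it casts player 0's character to ThirdPersonCharacter and calls EmergencyFlip.
; An unreachable leftover Launch timeline would raise a Princess character by LaunchDistance and then call its DeathEvent.
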(event `self.ReceiveActorBeginOverlap`
  (params (OtherActor :type "Actor Object Reference"))
  ;[1 1 1] Old logic, add begin overlap
  (if (`self.ActorHasTag` OtherActor "Player")
    (`/Game/ThirdPersonBP/Blueprints/ThirdPersonCharacter.EmergencyFlip` (cast `/Game/ThirdPersonBP/Blueprints/ThirdPersonCharacter` (`GameplayStatics.GetPlayerCharacter` 0) :!pure true))))

(fn `UserConstructionScript`)