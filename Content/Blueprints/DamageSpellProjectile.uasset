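; Spell projectile that deals a fixed amount of damage to an enemy it overlaps, then destroys itself.
; Overlap only counts for actors that pass a Damageable cast and carry the Enemy tag, and triggers a DealDamage message.
; Its DealDamage event casts the target to Enemy and calls ReceiveDamage, passing itself as a Damaging causer.
; BeginPlay, Hit and the construction script are empty.
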(event `self.ReceiveBeginPlay`)

(event `self.ReceiveActorBeginOverlap`
  (params (OtherActor :type "Actor Object Reference"))
  (bind _asdamageable (cast `/Game/Blueprints/Interfaces/Damageable` OtherActor))
  (if (`self.ActorHasTag` OtherActor "Enemy")
    (message `/Game/Blueprints/Interfaces/Damaging.DealDamage` self 0.65 _asdamageable)
    (`self.K2_DestroyActor`)))

(event `self.ReceiveHit`
  (params (MyComp :type "PrimitiveComponent Object Reference") (Other :type "Actor Object Reference") (OtherComp :type "PrimitiveComponent Object Reference") (bSelfMoved :type Boolean) (HitLocation :type "Vector Structure") (HitNormal :type "Vector Structure") (NormalImpulse :type "Vector Structure") (Hit :type "HitResult Structure (by ref)")))

(event `/Game/Blueprints/Interfaces/Damaging.DealDamage`
  (params (DamageAmount :type "Float (single-precision)") (Target :type "/Game/Blueprints/Interfaces/Damageable Interface"))
  (bind _asenemy (cast `/Game/Blueprints/Enemies/Enemy` Target))
  (bind _asdamaging (cast `/Game/Blueprints/Interfaces/Damaging` self))
  (`/Game/Blueprints/Enemies/Enemy.ReceiveDamage` _asenemy DamageAmount _asdamaging))

(fn `UserConstructionScript`)