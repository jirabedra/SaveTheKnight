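; A floating bullseye target that turns into a solid platform when hit by a PrincessProjectile.
; The construction script hides the Cube platform and disables its collision along with the Collision component.
; On overlap with a projectile, it destroys the projectile, reveals and enables the Cube and Collision, then hides the Cylinder and disables the Capsule and Box collision.
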(event `self.ReceiveBeginPlay`)

(event `self.ReceiveActorBeginOverlap`
  (params (OtherActor :type "Actor Object Reference"))
  (bind _asprincess_projectile (cast `/Game/Blueprints/PrincessProjectile` OtherActor))
  (`self.K2_DestroyActor` _asprincess_projectile)
  (`|ExecutionSequence`
    (:`then_0`
      (`SceneComponent.SetVisibility` (`self.Cube`) true false)
      (`PrimitiveComponent.SetCollisionEnabled` (`self.Collision`) "QueryAndPhysics")
      (`PrimitiveComponent.SetCollisionEnabled` (`self.Cube`) "QueryAndPhysics"))
    (:`then_1`
      (`SceneComponent.SetVisibility` (`self.Cylinder`) false false)
      (`PrimitiveComponent.SetCollisionEnabled` (`self.Capsule`) "NoCollision")
      (`PrimitiveComponent.SetCollisionEnabled` (`self.Box`) "NoCollision"))))

(fn `UserConstructionScript`
  (`SceneComponent.SetVisibility` (`self.Cube`) false false)
  (`PrimitiveComponent.SetCollisionEnabled` (`self.Collision`) "NoCollision")
  (`PrimitiveComponent.SetCollisionEnabled` (`self.Cube`) "NoCollision"))