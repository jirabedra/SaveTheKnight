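; ActivationLever is an interactable lever that toggles between activated and deactivated states.
; The Activate event flips the Activated flag and rotates the Handle mesh 90 degrees in the matching direction.
; When an actor tagged Player overlaps it, the handle gets a custom depth stencil highlight and an interaction message widget appears, both removed when the overlap ends.
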(event `/Game/Blueprints/Interfaces/Activable/Activable.Activate`
  (if (`self.Activated`)
    (set `self.Activated` false)
    (`SceneComponent.K2_AddLocalRotation` (`self.Handle`) (struct :`Pitch` 90.0) false false)
    (else
      (set `self.Activated` true)
      (`SceneComponent.K2_AddLocalRotation` (`self.Handle`) (struct :`Pitch` -90.0) false false))))

(event `self.ReceiveActorBeginOverlap`
  (params (OtherActor :type "Actor Object Reference"))
  (if (`self.ActorHasTag` OtherActor "Player")
    (`PrimitiveComponent.SetRenderCustomDepth` (`self.Handle`) true)
    (`PrimitiveComponent.SetCustomDepthStencilValue` (`self.Handle`) 1)
    (bind _returnvalue (`|CreateWidget` "/Game/UI/Widgets/SimpleButton1InteracionMessage.SimpleButton1InteracionMessage_C"))
    (`UserWidget.AddToViewport` _returnvalue 9)))

(event `self.ReceiveActorEndOverlap`
  (params (OtherActor :type "Actor Object Reference"))
  (if (`self.ActorHasTag` OtherActor "Player")
    (`PrimitiveComponent.SetRenderCustomDepth` (`self.Handle`) false)
    (`PrimitiveComponent.SetCustomDepthStencilValue` (`self.Handle`) 0)
    (`Widget.RemoveFromParent` (stale `self.ReceiveActorBeginOverlap` _returnvalue))))

(fn `UserConstructionScript`)