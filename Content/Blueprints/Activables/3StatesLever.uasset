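; Three-state lever actor, an activable that the author's notes intend for platforming puzzles.
; Activate steps the state up or down in a ping-pong, reversing direction at either end, rotating the handle and printing the new state.
; Overlapping its box outlines the handle via custom depth stencil, shows an interaction message widget, sets Triggered and calls the triggered event; leaving undoes this and calls the off event.
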(event `/Game/Blueprints/Interfaces/Activable/Activable.Activate`
  ;[1 1 1] Desagradable implementación del patrón state para una lever de 3 estados. Esta palanca se va a usar para implementar los puzzles de plataformas. espués voy a ver formas de emprolijar esto......
  (if (`self.IncreasingState`)
    (switch `/Game/Blueprints/Activables/3LeverStates` (`self.ActualState`)
      (:`NewEnumerator0`
        (set `self.ActualState` "NewEnumerator1")
        (`KismetSystemLibrary.PrintString` (`|GetEnumeratorNameAsString` (`self.ActualState`)))
        (`SceneComponent.K2_AddLocalRotation` (`self.Handle`) (struct :`Pitch` -45.0) false false))
      (:`NewEnumerator1`
        (set `self.ActualState` "NewEnumerator2")
        (`KismetSystemLibrary.PrintString` (`|GetEnumeratorNameAsString` (`self.ActualState`)))
        (`SceneComponent.K2_AddLocalRotation` (`self.Handle`) (struct :`Pitch` -45.0) false false)
        (set `self.IncreasingState` false :!label _label))
      (:`NewEnumerator2`
        (set `self.ActualState` "NewEnumerator2")
        (`KismetSystemLibrary.PrintString` (`|GetEnumeratorNameAsString` (`self.ActualState`)))
        (goto _label)))
    (else
      (switch `/Game/Blueprints/Activables/3LeverStates` (`self.ActualState`)
        (:`NewEnumerator0`
          (set `self.ActualState` "NewEnumerator0")
          (`KismetSystemLibrary.PrintString` (`|GetEnumeratorNameAsString` (`self.ActualState`)))
          (set `self.IncreasingState` true :!label _label_2))
        (:`NewEnumerator1`
          (set `self.ActualState` "NewEnumerator0")
          (`KismetSystemLibrary.PrintString` (`|GetEnumeratorNameAsString` (`self.ActualState`)))
          (`SceneComponent.K2_AddLocalRotation` (`self.Handle`) (struct :`Pitch` 45.0) false false)
          (goto _label_2))
        (:`NewEnumerator2`
          (set `self.ActualState` "NewEnumerator1")
          (`KismetSystemLibrary.PrintString` (`|GetEnumeratorNameAsString` (`self.ActualState`)))
          (`SceneComponent.K2_AddLocalRotation` (`self.Handle`) (struct :`Pitch` 45.0) false false))))))

(event `self.Box.OnComponentBeginOverlap`
  (params (OverlappedComponent :type "PrimitiveComponent Object Reference") (OtherActor :type "Actor Object Reference") (OtherComp :type "PrimitiveComponent Object Reference") (OtherBodyIndex :type Integer) (bFromSweep :type Boolean) (SweepResult :type "HitResult Structure (by ref)"))
  (`PrimitiveComponent.SetRenderCustomDepth` (`self.Handle`) true)
  (`PrimitiveComponent.SetCustomDepthStencilValue` (`self.Handle`) 1)
  (bind _returnvalue (`|CreateWidget` "/Game/UI/Widgets/LeverInteractionMessage.LeverInteractionMessage_C"))
  (`UserWidget.AddToViewport` _returnvalue 9)
  (set `self.Triggered` true)
  (`self.TriggeredEvent`))

(event `self.Box.OnComponentEndOverlap`
  (params (OverlappedComponent :type "PrimitiveComponent Object Reference") (OtherActor :type "Actor Object Reference") (OtherComp :type "PrimitiveComponent Object Reference") (OtherBodyIndex :type Integer))
  (`PrimitiveComponent.SetRenderCustomDepth` (`self.Handle`) false)
  (`PrimitiveComponent.SetCustomDepthStencilValue` (`self.Handle`) 0)
  (`Widget.RemoveFromParent` (stale `self.Box.OnComponentBeginOverlap` _returnvalue))
  (set `self.Triggered` false)
  (`self.TriggeredOffEvent`))

(fn `UserConstructionScript`)