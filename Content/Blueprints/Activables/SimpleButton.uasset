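; SimpleButton is an activable button actor that flips its Activated state each time Activate fires, nudging the Button component along its local Z axis to match.
; When an actor tagged Player overlaps it, the button enables custom depth with a stencil value and shows a display widget on screen.
; Ending the overlap clears the stencil and removes the widget.
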(event `/Game/Blueprints/Interfaces/Activable/Activable.Activate`
  (if (`self.Activated`)
    (set `self.Activated` false)
    (`SceneComponent.K2_AddLocalOffset` (`self.Button`) (0.0 0.0 -5.0) false false)
    (else
      (set `self.Activated` true)
      (`SceneComponent.K2_AddLocalOffset` (`self.Button`) (0.0 0.0 5.0) false false))))

(event `self.ReceiveActorBeginOverlap`
  (params (OtherActor :type "Actor Object Reference"))
  (if (`self.ActorHasTag` OtherActor "Player")
    (`PrimitiveComponent.SetRenderCustomDepth` (`self.Button`) true)
    (`PrimitiveComponent.SetCustomDepthStencilValue` (`self.Button`) 1)
    (bind _returnvalue (`|CreateWidget` (`self.DisplayWidgetBPClass`)))
    (`UserWidget.AddToViewport` _returnvalue 9)))

(event `self.ReceiveActorEndOverlap`
  (params (OtherActor :type "Actor Object Reference"))
  (if (`self.ActorHasTag` OtherActor "Player")
    (`PrimitiveComponent.SetRenderCustomDepth` (`self.Button`) false)
    (`PrimitiveComponent.SetCustomDepthStencilValue` (`self.Button`) 0)
    (`Widget.RemoveFromParent` (stale `self.ReceiveActorBeginOverlap` _returnvalue))))

(fn `UserConstructionScript`)