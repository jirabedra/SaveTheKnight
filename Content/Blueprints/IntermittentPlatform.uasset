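; IntermittentPlatform is a platform actor that repeatedly appears and disappears on a timed interval.
; Tick runs through a Delay of configurable length, which paces the toggle because calls made while it is pending are ignored.
; Each time the delay completes, IsCubeActive flips, switching the Cube's visibility and both the Cube's and Collision component's collision between off and query-and-physics.
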(event `self.ReceiveTick`
  (params (DeltaSeconds :type "Float (single-precision)"))
  (bind _cube (`self.Cube`))
  (bind _cube_2 (`self.Cube`))
  (`KismetSystemLibrary.Delay` (`self.Delay`))
  (if (`self.IsCubeActive`)
    (`SceneComponent.SetVisibility` _cube false false)
    (`PrimitiveComponent.SetCollisionEnabled` _cube "NoCollision")
    (`PrimitiveComponent.SetCollisionEnabled` (`self.Collision`) "NoCollision")
    (set `self.IsCubeActive` false)
    (else
      (`SceneComponent.SetVisibility` _cube_2 true false)
      (`PrimitiveComponent.SetCollisionEnabled` _cube_2 "QueryAndPhysics")
      (`PrimitiveComponent.SetCollisionEnabled` (`self.Collision`) "QueryAndPhysics")
      (set `self.IsCubeActive` true))))

(fn `UserConstructionScript`)