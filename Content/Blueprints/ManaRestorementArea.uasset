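; Mana restore pickup area that refills the Princess player's mana once, showing a Niagara cue from BeginPlay.
; On overlap, if not yet activated and the player Princess's mana is below 1.0, it passes the amount and itself to her NotifyManaRestorement.
; NotifyActivation, meant for when the restore succeeds, sets the one-shot flag, spawns the restore effect and destroys the actor after three seconds.
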(event `self.ReceiveBeginPlay`
  (`NiagaraFunctionLibrary.SpawnSystemAttached` "/Game/STKAssets/Particles/NiagaraSystems/NS_ManaRestorementVisualCue.NS_ManaRestorementVisualCue" (`self.NS`) "None" (0.0 0.0 0.0) (struct) "KeepRelativeOffset"))

(event `self.ReceiveActorBeginOverlap`
  (params (OtherActor :type "Actor Object Reference"))
  ;[0.1739 0.4226 1] precondiciones y notificacion a princesa
  (if (not (`self.bActivated`))
    (if (< (`/Game/ThirdPersonBP/Blueprints/Princess.Mana` (cast `/Game/ThirdPersonBP/Blueprints/Princess` (`GameplayStatics.GetPlayerCharacter` 0) :!pure true)) 1.0)
      (`/Game/ThirdPersonBP/Blueprints/Princess.NotifyManaRestorement` (cast `/Game/ThirdPersonBP/Blueprints/Princess` (`GameplayStatics.GetPlayerCharacter` 0) :!pure true) (`self.ManaAmountToRestore`) self))))

(event `NotifyActivation`
  ;[0.3585 0.6536 1] si el mana efectivamente pudo ser recuperado
  (if (not (`self.bActivated`))
    (set `self.bActivated` true)
    (`NiagaraFunctionLibrary.SpawnSystemAttached` "/Game/STKAssets/Particles/NiagaraSystems/NS_ManaRestorement.NS_ManaRestorement" (`self.NS`) "None" (0.0 0.0 0.0) (struct) "KeepRelativeOffset")
    (`KismetSystemLibrary.Delay` 3.0)
    (`self.K2_DestroyActor`)))

(fn `UserConstructionScript`)