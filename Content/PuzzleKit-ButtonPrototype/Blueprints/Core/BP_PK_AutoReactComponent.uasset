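; Puzzle kit component that automatically sends a chosen action to a list of target actors at a timed interval.
; A looping timer, started on BeginPlay or by event, calls PKDoAction on each target with the owner as instigator.
; It stops on request, at the loop limit (zero is unlimited), or when Action is None.
; Start and stop are authority-only, and helpers add or remove a stateful owner as a target.
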(event `self.ReceiveBeginPlay`
  ;[0 0 0] Start the timer
  (if (`self.bStartAutomatically`)
    (`self.PK_Start`)))

(event `PK_Start`
  ;[1 1 1] Create the timer and save the handle for later use
  (`self.HasAuthority`)
  (if (and (> (`KismetArrayLibrary.Array_Length` (`self.SendActionsTo`)) 0) (`|EnumInequality` (`self.Action`) "NewEnumerator9"))
    (set `self.Count` 0)
    (bind _returnvalue (`KismetSystemLibrary.K2_SetTimerDelegate` (delegate `PK_RunTimedAction`) (`self.Interval`) true))
    (set `self.Timer` _returnvalue)))

(event `PK_RunTimedAction`
  (bind _loop (`self.Loop`))
  ;[1 1 1] The timer loop: If Times is 0, or the maximum amout was reached, stop it, othewise send the selected action
  (if (or (and (>= (`self.Count`) _loop) (!= _loop 0)) (`|EnumEquality` (`self.Action`) "NewEnumerator9"))
    ;[1 1 1] Automatically stop if the limit is reached, or Action is None
    (`self.PK_Stop`)
    (else
      ;[1 1 1] Increment Count and send the selected Action to owner
      (set `self.Count` (+ (`self.Count`) 1))
      (for _array_element (`self.SendActionsTo`)
        (`/Engine/EditorBlueprintResources/StandardMacros.IsValid` _array_element
          (:`Is Valid`
            (`/Game/PuzzleKit-ButtonPrototype/Blueprints/Core/BP_PK_StatefulActor.PK_DoAction` _array_element (`self.Action`) (`self.GetOwner`))))))))

(event `PK_Stop`
  (bind _timer (`self.Timer`))
  ;[1 1 1] Clear and invalidate the timer
  (`self.HasAuthority`)
  (if (`KismetSystemLibrary.K2_IsValidTimerHandle` _timer)
    (`KismetSystemLibrary.K2_ClearAndInvalidateTimerHandle` _timer)))

(fn `OwnerIsPassive`
  (bind _returnvalue (`self.GetOwner`))
  (`/Engine/EditorBlueprintResources/StandardMacros.IsValid` _returnvalue
    (:`Is Valid`
      (bind _asbp_pk_stateful_actor (cast `/Game/PuzzleKit-ButtonPrototype/Blueprints/Core/BP_PK_StatefulActor` _returnvalue))
      (`KismetArrayLibrary.Array_RemoveItem` (`self.SendActionsTo`) _asbp_pk_stateful_actor))))

(fn `SendActionsToOwner`
  (bind _returnvalue (`self.GetOwner`))
  (`/Engine/EditorBlueprintResources/StandardMacros.IsValid` _returnvalue
    (:`Is Valid`
      (bind _asbp_pk_stateful_actor (cast `/Game/PuzzleKit-ButtonPrototype/Blueprints/Core/BP_PK_StatefulActor` _returnvalue))
      ;[1 1 1] Add owner to SendActionsTo
      (`KismetArrayLibrary.Array_AddUnique` (`self.SendActionsTo`) _asbp_pk_stateful_actor))
    (:`Is Not Valid`
      ;[0 0 0] Log DebugMessage if owner is not stateful
      (`/Game/PuzzleKit-ButtonPrototype/Blueprints/Core/BPL_PK_LogFunction.PK_ErrorLogMessage` "Owner is not a BP_PK_StatefulActor, so it cannot trigger state change events." self))))