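; Puzzle-kit component that observes state changes on ListenTo stateful actors and reacts by sending actions to SendActionsTo actors, server-side.
; Changes are queued, optionally delayed, then stored in a state buffer by passthrough, per-actor aggregation or rolling history.
; The first rule matching the buffer tail, with wildcards, and change reason picks the action, propagated at reduced MaxPropagation to limit chains.
; It can also forward changes and failures to its owner.
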(event `self.ReceiveBeginPlay`
  (bind _returnvalue (`self.GetOwner`))
  (bind _returnvalue_2 (`self.GetOwner`))
  (`/Engine/EditorBlueprintResources/StandardMacros.IsValid` _returnvalue_2
    (:`Is Valid`
      (if (`Actor.HasAuthority` _returnvalue_2)
        (`|ExecutionSequence`
          (:`then_0`
            ;[0 0 0] Check if owner is observer and can receive State Events
            (`/Engine/EditorBlueprintResources/StandardMacros.IsValid` _returnvalue
              (:`Is Valid`
                (if (and (`self.bSendEventsToObserverOwner`) (not (`.bSuccess` (cast `/Game/PuzzleKit-ButtonPrototype/Blueprints/Core/BPI_PK_ObserverActor` _returnvalue :!pure true))))
                  (`/Game/PuzzleKit-ButtonPrototype/Blueprints/Core/BPL_PK_LogFunction.PK_ErrorLogMessage` "Owner is not a BPI_PK_StateObserver. It will not receive State events." self)))))
          (:`then_1`
            ;[1 1 1] If should aggregate events, then collect all initial states from the observed actors
            (if (`|EnumEquality` (`self.OnStateChanged`) "NewEnumerator1")
              (`self.AggregateInitialStates`)))
          (:`then_2`
            ;[1 1 1] Calculate maximum buffer size based on longest state match rule.
            (if (and (`self.bBufferMaxSizeToLongestRule`) (`self.bEnableReactions`))
              (set `self.BufferMaxSize` 0)
              (for _array_element (`self.Rules`)
                (bind _statearray (`self.StringAsStatesArray` (break `/Game/PuzzleKit-ButtonPrototype/Blueprints/Core/Structs/FPKChangeReaction` _array_element)))
                (set `self.BufferMaxSize` (`KismetMathLibrary.Max` (`KismetArrayLibrary.Array_Length` _statearray) (`self.BufferMaxSize`))))))
          (:`then_3`
            ;[1 1 1] Set default private variable values
            (set `self.bIsBusy` false))
          (:`then_4`
            ;[1 1 1] Bind to IterativeState component of actor
            (for _array_element_2 (`self.ListenTo`)
              (bind _statecomponent (`self.HasValidStateComponent` _array_element_2)
                (:`Is Valid`
                  (`|ExecutionSequence`
                    (:`then_0`
                      ;[0.5833 1 0.6334] State Change Success
                      (if (`self.bObserveStateChanges`)
                        (add `/Game/PuzzleKit-ButtonPrototype/Blueprints/Core/BP_PK_IterativeStateComponent.OnStateChanged` _statecomponent (delegate `HandleOnStateChanged`))))
                    (:`then_1`
                      ;[1 0.5573 0.5573] State Change Failure
                      (if (`self.bObserveChangeFailures`)
                        (add `/Game/PuzzleKit-ButtonPrototype/Blueprints/Core/BP_PK_IterativeStateComponent.OnStateFailure` _statecomponent (delegate `HandleObservedFailure`))))))))))))))

(event `HandleOnStateChanged_Inner`
  (bind _returnvalue (`self.GetOwner`))
  (bind _reactionsdelay (`self.ReactionsDelay`))
  ;[0.5833 1 0.6334] State Change Success
  (set `self.bIsBusy` true)
  (if (> _reactionsdelay 0.0)
    (`KismetSystemLibrary.Delay` _reactionsdelay))
  (bind (_bisvalid _output) (`self.GetFromQueue`))
  (if _bisvalid
    (`|ExecutionSequence`
      (:`then_0`
        (bind (_state _sender _instigator _reason _maxpropagation) (break `/Game/PuzzleKit-ButtonPrototype/Blueprints/Core/Structs/FPKStateChangeArgs` _output))
        (`self.ProcessNewState` _state _sender)
        ;;[1 1 1] Try to call owner success events, with processed state
        (if (and (`self.bSendEventsToObserverOwner`) (`KismetSystemLibrary.IsValid` _returnvalue))
          (message `/Game/PuzzleKit-ButtonPrototype/Blueprints/Core/BPI_PK_ObserverActor.PK_HandleStateChanged` _returnvalue (make `/Game/PuzzleKit-ButtonPrototype/Blueprints/Core/Structs/FPKStateChangeArgs` (`self.StatesArrayAsString` (`self.StatesBuffer`)) self _instigator _reason _maxpropagation)))
        ;;[1 1 1] Propagate action only if it has enough life
        (if (and (`self.bEnableReactions`) (>= _maxpropagation (`self.PropagationCost`)))
          (bind (_btranslationfound _action) (`self.TryMatchRule` _reason))
          (if _btranslationfound
            ;;[1 1 1] If Propagation Rule found, send action to actors, and then clear buffer (if necessary)
            (if (`self.bBufferClearOnRuleMatch`)
              (`self.ClearBuffer`))
            (if (> (`KismetArrayLibrary.Array_Length` (`self.SendActionsTo`)) 0)
              (for _array_element (`self.SendActionsTo`)
                ;;[1 1 1] Send actions to all actors that have a valid state component
                (bind _statecomponent (`self.HasValidStateComponent` _array_element)
                  (:`Is Valid`
                    (bind _bsuccess (`/Game/PuzzleKit-ButtonPrototype/Blueprints/Core/BP_PK_IterativeStateComponent.DoActionPropagated` _statecomponent _action _instigator (- _maxpropagation (`self.PropagationCost`))))
                    (if (and (not _bsuccess) (`self.bStopOnFirstFailure`))
                      (break)))))))))
      (:`then_1`
        ;[1 1 1] ClearBuffer
        (if (> (`self.BufferAutoClearDelay`) 0.0)
          (`KismetSystemLibrary.K2_SetTimer` self "ClearBufferWithEvents" (`self.BufferAutoClearDelay`))))
      (:`then_2`
        (if (`self.QueueHasItems`)
          (`self.HandleOnStateChanged_Inner`)
          (else
            (set `self.bIsBusy` false)))))))

(event `HandleOnStateChanged`
  (params (State :type "/Game/PuzzleKit-ButtonPrototype/Blueprints/Core/Structs/FPKStateChangeArgs Structure"))
  ;[0.5833 1 0.6334] State Change Success
  (`self.HasAuthority`
    (:`OnAuthority`
      (`self.AddToQueue` State)
      (`self.HandleOnStateChanged_Inner`))))

(event `HandleObservedFailure`
  (params (ErrorArgs :type "/Game/PuzzleKit-ButtonPrototype/Blueprints/Core/Structs/FPKStateChangeArgs Structure") (FailReason :type "/Game/PuzzleKit-ButtonPrototype/Blueprints/Core/Enums/EPK_FailReason Enum" :default "NewEnumerator3"))
  (bind _returnvalue (`self.GetOwner`))
  ;[1 0.5573 0.5573] State Change Failure
  (if (and (`self.bSendEventsToObserverOwner`) (`KismetSystemLibrary.IsValid` _returnvalue))
    (message `/Game/PuzzleKit-ButtonPrototype/Blueprints/Core/BPI_PK_ObserverActor.PK_HandleChangeFailure` _returnvalue (make `/Game/PuzzleKit-ButtonPrototype/Blueprints/Core/Structs/FPKStateChangeArgs` ErrorArgs_State_56_430119DD4B18CA4282D828BECAA4FD60 self ErrorArgs_Instigator_84_AD3B4C2B4AE092498541D88B70385490 ErrorArgs_Reason_71_B758D633491B7A72BAA4FAAAD8C78C7E ErrorArgs_MaxPropagation_85_6B587002433AF8E4FCC0A0B8B071BE36) FailReason)))

(fn `ActionMappingToAction`
  (params (Mapping :type "/Game/PuzzleKit-ButtonPrototype/Blueprints/Core/Enums/EPK_StateActionMapping Enum" :default "NewEnumerator7") (ChangeReason :type "/Game/PuzzleKit-ButtonPrototype/Blueprints/Core/Enums/EPK_StateAction Enum" :default "NewEnumerator9"))
  (returns (Action :type "/Game/PuzzleKit-ButtonPrototype/Blueprints/Core/Enums/EPK_StateAction Enum"))
  (return (select `/Game/PuzzleKit-ButtonPrototype/Blueprints/Core/Enums/EPK_StateActionMapping` Mapping :`NewEnumerator7` "NewEnumerator9" :`NewEnumerator3` "NewEnumerator3" :`NewEnumerator4` "NewEnumerator4" :`NewEnumerator5` "NewEnumerator5" :`NewEnumerator8` "NewEnumerator8" :`NewEnumerator9` ChangeReason)))

(fn `ActionToActionMapping`
  (params (Action :type "/Game/PuzzleKit-ButtonPrototype/Blueprints/Core/Enums/EPK_StateAction Enum" :default "NewEnumerator9"))
  (returns (Mapping :type "/Game/PuzzleKit-ButtonPrototype/Blueprints/Core/Enums/EPK_StateActionMapping Enum"))
  (return (select `/Game/PuzzleKit-ButtonPrototype/Blueprints/Core/Enums/EPK_StateAction` Action :`NewEnumerator9` "NewEnumerator7" :`NewEnumerator3` "NewEnumerator3" :`NewEnumerator4` "NewEnumerator4" :`NewEnumerator5` "NewEnumerator5" :`NewEnumerator8` "NewEnumerator8" :!type "/Game/PuzzleKit-ButtonPrototype/Blueprints/Core/Enums/EPK_StateActionMapping Enum")))

(fn `AddStateToBuffer`
  (params (NewState :type String))
  ;[1 1 1] Adds new state to the end of the buffer and adjust buffer size (if necessary)
  (bind _returnvalue (`KismetArrayLibrary.Array_Add` (`self.StatesBuffer`) NewState))
  (if (>= _returnvalue (`self.BufferMaxSize`))
    (`KismetArrayLibrary.Array_Remove` (`self.StatesBuffer`))))

(fn `AddToQueue`
  (params (NewItem :type "/Game/PuzzleKit-ButtonPrototype/Blueprints/Core/Structs/FPKStateChangeArgs Structure (by ref)"))
  (`KismetArrayLibrary.Array_Add` (`self.SuccessEventsQueue`) NewItem))

(fn `AggregateInitialStates`
  (locals (CollectedStates :type "Array of String"))
  ;[1 1 1] Collects initial stated for all observed actors. If the ListenTo contains empty elements, it will collect empty strings.
  (for (_array_element _array_index) (`self.ListenTo`)
    (`/Engine/EditorBlueprintResources/StandardMacros.IsValid` _array_element
      (:`Is Valid`
        (bind _returnvalue (`Actor.GetComponentByClass` _array_element "/Game/PuzzleKit-ButtonPrototype/Blueprints/Core/BP_PK_IterativeStateComponent.BP_PK_IterativeStateComponent_C"))
        (`/Engine/EditorBlueprintResources/StandardMacros.IsValid` _returnvalue
          (:`Is Valid`
            (bind (_state _bvalid) (`/Game/PuzzleKit-ButtonPrototype/Blueprints/Core/BP_PK_IterativeStateComponent.TryGetState` _returnvalue (`/Game/PuzzleKit-ButtonPrototype/Blueprints/Core/BP_PK_IterativeStateComponent.StartupStateId` _returnvalue)))
            (if _bvalid
              (`KismetArrayLibrary.Array_Set` (`local.CollectedStates`) _array_index _state true)))))))
  (set `self.StatesBuffer` (`local.CollectedStates`))
  (return))

(fn `AggregateStates`
  (params (NewState :type String) (Sender :type "ActorComponent Object Reference"))
  (locals (CollectedStates :type "Array of String"))
  (bind _returnvalue (`self.GetOwner` Sender))
  ;[1 1 1] Insert the state in the StatesBuffer array, at the same index as the sender actor index, from ListenTo array
  (`/Engine/EditorBlueprintResources/StandardMacros.IsValid` Sender
    (:`Is Valid`
      (`/Engine/EditorBlueprintResources/StandardMacros.IsValid` _returnvalue
        (:`Is Valid`
          (bind _asbp_pk_stateful_actor (cast `/Game/PuzzleKit-ButtonPrototype/Blueprints/Core/BP_PK_StatefulActor` _returnvalue))
          (bind _returnvalue_2 (`KismetArrayLibrary.Array_Find` (`self.ListenTo`) _asbp_pk_stateful_actor))
          (if (>= _returnvalue_2 0)
            (`KismetArrayLibrary.Array_Set` (`self.StatesBuffer`) _returnvalue_2 (`local.NewState`) true)))))))

(fn `ClearBuffer`
  ;[1 1 1] Clears the buffer, but only if it is AddToBuffer
  (if (`|EnumEquality` (`self.OnStateChanged`) "NewEnumerator2")
    (`KismetArrayLibrary.Array_Clear` (`self.StatesBuffer`))))

(fn `ClearBufferWithEvents`
  (bind _returnvalue (`self.GetOwner`))
  ;[1 1 1] Clears the buffer, but only if it is AddToBuffer
  (`self.ClearBuffer`)
  (if (and (`self.bSendEventsToObserverOwner`) (`KismetSystemLibrary.IsValid` _returnvalue))
    (message `/Game/PuzzleKit-ButtonPrototype/Blueprints/Core/BPI_PK_ObserverActor.PK_HandleStateChanged` _returnvalue (make `/Game/PuzzleKit-ButtonPrototype/Blueprints/Core/Structs/FPKStateChangeArgs` "" self _returnvalue "NewEnumerator9" 0))))

(fn `GetFromQueue`
  (returns (bIsValid :type Boolean) (Output :type "/Game/PuzzleKit-ButtonPrototype/Blueprints/Core/Structs/FPKStateChangeArgs Structure (by ref)"))
  (locals (Item :type "/Game/PuzzleKit-ButtonPrototype/Blueprints/Core/Structs/FPKStateChangeArgs Structure"))
  (bind _successeventsqueue (`self.SuccessEventsQueue`))
  (if (`self.QueueHasItems`)
    (set `local.Item` (`|GetArrayItem` _successeventsqueue))
    (`KismetArrayLibrary.Array_Remove` _successeventsqueue)
    (return true (`local.Item`))))

(fn `ListenToOwner`
  (locals (StatefulOwner :type "/Game/PuzzleKit-ButtonPrototype/Blueprints/Core/BP_PK_StatefulActor Object Reference"))
  (bind _asbp_pk_stateful_base (`self.AsStateful` (`self.GetOwner`))
    (:`then`
      ;[1 1 1] Add owner to ListenTo and Remove it from SendActionsTo array
      (bind _output_get (set `local.StatefulOwner` _asbp_pk_stateful_base))
      (`KismetArrayLibrary.Array_AddUnique` (`self.ListenTo`) _output_get)
      (`KismetArrayLibrary.Array_RemoveItem` (`self.SendActionsTo`) (`local.StatefulOwner`)))
    (:`CastFailed`
      ;[0 0 0] Log debug message if owner is not stateful
      (`/Game/PuzzleKit-ButtonPrototype/Blueprints/Core/BPL_PK_LogFunction.PK_ErrorLogMessage` "Owner is not a BP_PK_StatefulActor, so it cannot receive state change actions." self))))

(fn `OwnerIsPassive`
  (bind _asbp_pk_stateful_base (`self.AsStateful` (`self.GetOwner`))
    (:`then`
      ;[1 1 1] Remove owner from ListenTo and SendActionsTo
      (`KismetArrayLibrary.Array_RemoveItem` (`self.ListenTo`) _asbp_pk_stateful_base)
      (`KismetArrayLibrary.Array_RemoveItem` (`self.SendActionsTo`) _asbp_pk_stateful_base))))

(fn `PassthroughState`
  (params (NewState :type String))
  (locals (CollectedStates :type "Array of String"))
  ;[1 1 1] The new state is immediatly passed over, thus the buffer will only have this element
  (set `self.StatesBuffer` (`|MakeArray` NewState))
  (return))

(fn `PK_GetBuffer`
  (returns (Buffer :type "Array of String"))
  (return (`self.StatesBuffer`)))

(fn `PK_IsBusy`
  (returns (bIsBusy :type Boolean))
  (return (`self.bIsBusy`)))

(fn `ProcessNewState`
  (params (State :type String) (Sender :type "ActorComponent Object Reference"))
  ;[1 1 1] According to state collection strategy (OnStateChange enum) adds the current state to the state buffer
  (switch `/Game/PuzzleKit-ButtonPrototype/Blueprints/Core/Enums/EPK_AggregationStrategy` (`self.OnStateChanged`)
    (:`NewEnumerator3`
      (`self.PassthroughState` State))
    (:`NewEnumerator1`
      (`self.AggregateStates` State Sender))
    (:`NewEnumerator2`
      (`self.AddStateToBuffer` State))))

(fn `QueueHasItems`
  (returns (ReturnValue :type Boolean))
  (return (> (`KismetArrayLibrary.Array_Length` (`self.SuccessEventsQueue`)) 0)))

(fn `SendActionToOwner`
  (locals (StatefulOwner :type "/Game/PuzzleKit-ButtonPrototype/Blueprints/Core/BP_PK_StatefulActor Object Reference"))
  (bind _asbp_pk_stateful_base (`self.AsStateful` (`self.GetOwner`))
    (:`then`
      ;[1 1 1] Add owner to SendActionsTo and Remove it from ListenTo array
      (bind _output_get (set `local.StatefulOwner` _asbp_pk_stateful_base))
      (`KismetArrayLibrary.Array_AddUnique` (`self.SendActionsTo`) _output_get)
      (`KismetArrayLibrary.Array_RemoveItem` (`self.ListenTo`) (`local.StatefulOwner`)))
    (:`CastFailed`
      ;[0 0 0] Log DebugMessage if owner is not stateful
      (`/Game/PuzzleKit-ButtonPrototype/Blueprints/Core/BPL_PK_LogFunction.PK_ErrorLogMessage` "Owner is not a BP_PK_StatefulActor, so it cannot trigger state change events." self))))

(fn `StatesArrayAsString`
  (params (States :type "Array of String"))
  (returns (ReturnValue :type String))
  (return (`KismetStringLibrary.JoinStringArray` States (`self.StateSeparator`))))

(fn `StringAsStatesArray`
  (params (State :type String))
  (returns (StateArray :type "Array of String"))
  (return (`KismetStringLibrary.ParseIntoArray` State (`self.StateSeparator`) false)))

(fn `TryMatchRule`
  (params (StateChangeReason :type "/Game/PuzzleKit-ButtonPrototype/Blueprints/Core/Enums/EPK_StateAction Enum" :default "NewEnumerator9"))
  (returns (bTranslationFound :type Boolean) (Action :type "/Game/PuzzleKit-ButtonPrototype/Blueprints/Core/Enums/EPK_StateAction Enum"))
  (locals (bFoundTranslation :type Boolean) (TranslationCandidate :type "/Game/PuzzleKit-ButtonPrototype/Blueprints/Core/Structs/FPKChangeReaction Structure") (StartIndex :type Integer) (ActionCandidate :type "/Game/PuzzleKit-ButtonPrototype/Blueprints/Core/Enums/EPK_StateAction Enum"))
  ;[0 0 0] Searches all translations, first by matching the action that triggered the state change, then by matching the state strings, accounting for the wildcards
  ;;[1 1 1] Search all translations
  (for _array_element (`self.Rules`)
    (bind _output_get (set `local.TranslationCandidate` _array_element))
    ;;[1 1 1] Try and find a matching action for the ChangeReason action. First check for Any, and then check for exact action
    (if (or (`|EnumEquality` (`.AndWasChangedBy_99_E6B718064F3FA9FF016A9B962A26A136` (break `/Game/PuzzleKit-ButtonPrototype/Blueprints/Core/Structs/FPKChangeReaction` _output_get)) "NewEnumerator9") (`|EnumEquality` (`.AndWasChangedBy_99_E6B718064F3FA9FF016A9B962A26A136` (break `/Game/PuzzleKit-ButtonPrototype/Blueprints/Core/Structs/FPKChangeReaction` _output_get)) (`self.ActionToActionMapping` (`local.StateChangeReason`))))
      (set `local.ActionCandidate` (`self.ActionMappingToAction` (`.DoAction_96_BF1C12D64E9D0AA694B380A5D6B05A3D` (break `/Game/PuzzleKit-ButtonPrototype/Blueprints/Core/Structs/FPKChangeReaction` _output_get)) (`local.StateChangeReason`)))
      ;;[1 1 1] Split translation by delimiter
      (bind _statearray (`self.StringAsStatesArray` (break `/Game/PuzzleKit-ButtonPrototype/Blueprints/Core/Structs/FPKChangeReaction` _output_get)))
      ;;[1 1 1] If translation is longer than buffer size, don't even try to translae
      (bind _output_get_2 (set `local.StartIndex` (- (`KismetArrayLibrary.Array_Length` (`self.StatesBuffer`)) (`KismetArrayLibrary.Array_Length` _statearray))))
      (if (>= _output_get_2 0)
        (set `local.bFoundTranslation` true)
        (for _index (range (+ (`KismetArrayLibrary.Array_LastIndex` _statearray) 1))
          (bind _output (`|GetArrayItem` _statearray _index))
          ;;[1 1 1] Compare items one by one, and break at first mismatch
          (if (and (`KismetStringLibrary.NotEqual_StrStr` (`self.StateWildcard`) _output) (`KismetStringLibrary.NotEqual_StrStr` _output (`|GetArrayItem` (`self.StatesBuffer`) (+ (`local.StartIndex`) _index))))
            (set `local.bFoundTranslation` false)
            (break)))
        ;;[1 1 1] Return first found translation
        (if (`local.bFoundTranslation`)
          (return true (`local.ActionCandidate`))))))
  ;;[1 1 1] If translation array reached the end, and no translation was found, return
  (return false "NewEnumerator9"))