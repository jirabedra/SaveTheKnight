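; Puzzle-kit actor component that holds an index into a list of named states and steps through it on action requests.
; Actions run only with authority, pass a blocked-events check and an accepted-action bitmask, then move the replicated state ID forward, back, or to a reset point.
; Stepping clamps, cycles or reverses direction at the ends.
; Change and failure dispatchers report results with instigator and propagation limit, optionally auto-bound to an observer-interface owner.
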(event `self.ReceiveBeginPlay`
  (bind _returnvalue (`self.GetOwner`))
  (bind _startupstateid (`self.StartupStateId`))
  ;[1 1 1] Event BeginPlay
  (`self.HasAuthority`
    (:`OnAuthority`
      (`|ExecutionSequence`
        (:`then_0`
          ;[0 0 0] Check if owner is observer and can receive State Events
          (`/Engine/EditorBlueprintResources/StandardMacros.IsValid` _returnvalue
            (:`Is Valid`
              (if (and (`self.bSendChangeEventsToObserverOwner`) (not (`.bSuccess` (cast `/Game/PuzzleKit-ButtonPrototype/Blueprints/Core/BPI_PK_ObserverActor` _returnvalue :!pure true))))
                (`/Game/PuzzleKit-ButtonPrototype/Blueprints/Core/BPL_PK_LogFunction.PK_ErrorLogMessage` "Owner is not a BPI_PK_StateObserver. It will  not receive state change events." self)))))
        (:`then_1`
          ;;[1 1 1] Set Default values
          (set `self.IncrementDirection` 1)
          (set `self.bCanReceiveEvents` true)
          ;;[1 1 1] Sets the state to the starting state
          (if (`self.IsStateIdValid` _startupstateid)
            (set `self.StateId` _startupstateid)
            (else
              ;;[0 0 0] Debug log invalid startup state
              (`/Game/PuzzleKit-ButtonPrototype/Blueprints/Core/BPL_PK_LogFunction.PK_ErrorLogMessage` "Invalid Startup State Id" self))))
        (:`then_2`
          ;;[1 1 1] Autobind owner, if it is an observer and the autobind flag is set
          (if (and (`self.bSendChangeEventsToObserverOwner`) (`KismetSystemLibrary.DoesImplementInterface` (`self.GetOwner`) "/Game/PuzzleKit-ButtonPrototype/Blueprints/Core/BPI_PK_ObserverActor.BPI_PK_ObserverActor_C"))
            ;;;[0.5833 1 0.6334] Bind Success Event
            (add `self.OnStateChanged` (delegate `CallSuccessOnOwner`))))
        (:`then_3`
          (if (and (`self.bSendFailureEventsToObserverOwner`) (`KismetSystemLibrary.DoesImplementInterface` (`self.GetOwner`) "/Game/PuzzleKit-ButtonPrototype/Blueprints/Core/BPI_PK_ObserverActor.BPI_PK_ObserverActor_C"))
            ;;;[1 0.5573 0.5573] Bind to Failure Event
            (add `self.OnStateFailure` (delegate `CallFailureOnOwner`))))))))

(event `CallSuccessOnOwner` :!signature `self.OnStateChanged`
  (params (State :type "/Game/PuzzleKit-ButtonPrototype/Blueprints/Core/Structs/FPKStateChangeArgs Structure"))
  ;[1 1 1] Event BeginPlay
  ;;[1 1 1] Autobind owner, if it is an observer and the autobind flag is set
  ;;;[0.5833 1 0.6334] Bind Success Event
  (message `/Game/PuzzleKit-ButtonPrototype/Blueprints/Core/BPI_PK_ObserverActor.PK_HandleStateChanged` (`self.GetOwner`) State))

(event `CallFailureOnOwner` :!signature `self.OnStateFailure`
  (params (ErrorArgs :type "/Game/PuzzleKit-ButtonPrototype/Blueprints/Core/Structs/FPKStateChangeArgs Structure") (FailReason :type "/Game/PuzzleKit-ButtonPrototype/Blueprints/Core/Enums/EPK_FailReason Enum" :default "NewEnumerator3"))
  ;[1 1 1] Event BeginPlay
  ;;[1 1 1] Autobind owner, if it is an observer and the autobind flag is set
  ;;;[1 0.5573 0.5573] Bind to Failure Event
  (message `/Game/PuzzleKit-ButtonPrototype/Blueprints/Core/BPI_PK_ObserverActor.PK_HandleChangeFailure` (`self.GetOwner`) ErrorArgs FailReason))

(event `PK_DoAction`
  (params (Action :type "/Game/PuzzleKit-ButtonPrototype/Blueprints/Core/Enums/EPK_StateAction Enum" :default "NewEnumerator9") (Instigator :type "Actor Object Reference"))
  ;[1 1 1] Delegate DoAction commands
  (`self.ExcecuteAction` Action Instigator (`self.MaxPropagation`)))

(fn `AutoIncrementState`
  (params (IncrementStep :type Integer))
  (returns (NextStateId :type Byte) (NextIncrementDirection :type Integer))
  (locals (NewStateId :type Integer) (bTriggerStateChangeOnSameState :type Boolean) (MaxStateId :type Integer) (NewIncrementDirection :type Integer))
  (bind _maxstateid (`local.MaxStateId`))
  (bind _newstateid (`local.NewStateId`))
  (bind _returnvalue (`KismetMathLibrary.SignOfInteger` (`local.IncrementStep`)))
  (set `local.NewIncrementDirection` (`self.IncrementDirection`))
  (bind _output_get (set `local.MaxStateId` (`KismetMathLibrary.Conv_ByteToInt` (`self.GetMaxStateId`))))
  ;[1 1 1] If we have only one state, return that state
  (if (== _output_get 0)
    (return 0 0)
    (else
      ;[1 1 1] Compute next state based on increment direction
      (set `local.NewStateId` (+ (`KismetMathLibrary.Conv_ByteToInt` (`self.StateId`)) (* IncrementStep (`self.IncrementDirection`))))
      (switch `/Game/PuzzleKit-ButtonPrototype/Blueprints/Core/Enums/EPK_StateResetBehaviour` (`self.IterateBehaviour`)
        (:`NewEnumerator0`
          ;[1 1 1] Blocked Behaviour
          (set `local.NewStateId` (`KismetMathLibrary.Clamp` (`local.NewStateId`) 0 (`local.MaxStateId`))))
        (:`NewEnumerator2`
          ;[1 1 1] Cycle Behaviour
          (set `local.NewStateId` (select `bool` (< (`local.NewStateId`) 0) :`false` (select `bool` (> _newstateid _maxstateid) :`false` _newstateid) :`true` _maxstateid)))
        (:`NewEnumerator1`
          ;[1 1 1] Reverse Behaviour
          (if (> (`local.NewStateId`) (`local.MaxStateId`))
            (set `local.NewIncrementDirection` (* _returnvalue -1))
            (set `local.NewStateId` (- (`local.MaxStateId`) 1))
            (elif (< (`local.NewStateId`) 0)
              (set `local.NewIncrementDirection` _returnvalue)
              (set `local.NewStateId` 1)))))
      (return (`KismetMathLibrary.Conv_IntToByte` (`local.NewStateId`)) (`local.NewIncrementDirection`)))))

(fn `BlockEvents`
  (set `self.bCanReceiveEvents` false))

(fn `CanExecuteAction`)

(fn `CanSetState`
  (returns (bCanSetState :type Boolean))
  (return (`self.bCanReceiveEvents`)))

(fn `DoActionPropagated`
  (params (Action :type "/Game/PuzzleKit-ButtonPrototype/Blueprints/Core/Enums/EPK_StateAction Enum" :default "NewEnumerator9") (Instigator :type "Actor Object Reference") (MaxPropagation :type Byte))
  (returns (bSuccess :type Boolean))
  (bind _bsuccess (`self.ExcecuteAction` Action Instigator (`KismetMathLibrary.BMin` MaxPropagation (`self.MaxPropagation`))))
  (return _bsuccess))

(fn `ExcecuteAction`
  (params (ChangedBy :type "/Game/PuzzleKit-ButtonPrototype/Blueprints/Core/Enums/EPK_StateAction Enum" :default "NewEnumerator9") (Instigator :type "Actor Object Reference") (MaxPropagation :type Byte))
  (returns (bSuccess :type Boolean))
  (locals (oldStateId :type Byte))
  (`self.HasAuthority`
    (:`OnAuthority`
      (if (`self.CanSetState`)
        (set `self.FailReason` "NewEnumerator3")
        (if (`self.IsSupprtedAction` ChangedBy)
          (bind (_nextstate _nextincrementdirection) (`self.SetNextState` ChangedBy))
          (bind (_state _bvalid) (`self.TryGetState` _nextstate))
          (if _bvalid
            (set `local.oldStateId` (`self.StateId`))
            ;[0.1473 0.6403 1] Set replicated variable
            (set `self.StateId` _nextstate)
            (set `self.IncrementDirection` _nextincrementdirection)
            (if (`self.ShouldFireChangedEvents` _nextstate (`local.oldStateId`))
              ;[0.5833 1 0.6334] Success
              (`self.OnStateChanged` (make `/Game/PuzzleKit-ButtonPrototype/Blueprints/Core/Structs/FPKStateChangeArgs` _state self Instigator ChangedBy MaxPropagation))
              (return true)
              (else
                ;[1 0.5573 0.5573] Go to state change failure
                (set `self.FailReason` "NewEnumerator2")))
            (else
              (set `self.FailReason` "NewEnumerator1")))
          (else
            (set `self.FailReason` "NewEnumerator0")))
        (else
          (set `self.FailReason` "NewEnumerator4")))
      ;[1 0.5573 0.5573] Call state failure
      (`self.OnStateFailure` (make `/Game/PuzzleKit-ButtonPrototype/Blueprints/Core/Structs/FPKStateChangeArgs` "" self Instigator ChangedBy MaxPropagation) (`self.FailReason`))
      (return false))))

(fn `GetMaxStateId`
  (returns (MaxStateId :type Byte))
  (return (`KismetMathLibrary.Conv_IntToByte` (`KismetArrayLibrary.Array_LastIndex` (`self.States`)))))

(fn `GetState`
  (returns (StateInfo :type String) (StateId :type Byte) (bIsValid :type Boolean))
  (bind _stateid (`self.StateId`))
  (bind (_state _bvalid) (`self.TryGetState` _stateid))
  ;[1 1 1] This function is needed, as the State variable is private
  (return _state _stateid _bvalid))

(fn `IsStateIdValid`
  (params (StateId :type Byte))
  (returns (bStateValid :type Boolean))
  (return (`KismetArrayLibrary.Array_IsValidIndex` (`self.States`) (`KismetMathLibrary.Conv_ByteToInt` StateId))))

(fn `IsSupprtedAction`
  (params (Action :type "/Game/PuzzleKit-ButtonPrototype/Blueprints/Core/Enums/EPK_StateAction Enum" :default "NewEnumerator9"))
  (returns (IsSupported :type Boolean))
  (locals (BitmaskAction :type Integer))
  (bind _output_get (set `local.BitmaskAction` (select `/Game/PuzzleKit-ButtonPrototype/Blueprints/Core/Enums/EPK_StateAction` Action :`NewEnumerator9` (`|BitmaskLiteral` 1) :`NewEnumerator3` (`|BitmaskLiteral` 2) :`NewEnumerator4` (`|BitmaskLiteral` 4) :`NewEnumerator5` (`|BitmaskLiteral` 8) :`NewEnumerator8` (`|BitmaskLiteral` 0))))
  (return (== _output_get (`KismetMathLibrary.And_IntInt` _output_get (`self.AcceptedActions`)))))

(fn `SetNextState`
  (params (Action :type "/Game/PuzzleKit-ButtonPrototype/Blueprints/Core/Enums/EPK_StateAction Enum" :default "NewEnumerator9"))
  (returns (NextState :type Byte) (NextIncrementDirection :type Integer))
  (locals (TmpState :type Byte) (TmpIncrementDirection :type Integer))
  (switch `/Game/PuzzleKit-ButtonPrototype/Blueprints/Core/Enums/EPK_StateAction` Action
    (:`NewEnumerator3`
      ;[1 1 1] Goes to next state, based on auto increment behaviour
      (bind (_nextstateid _nextincrementdirection) (`self.AutoIncrementState` 1))
      (set `local.TmpState` _nextstateid)
      (set `local.TmpIncrementDirection` _nextincrementdirection))
    (:`NewEnumerator4`
      ;[1 1 1] Goes to previous state, based on auto increment behaviour
      (bind (_nextstateid_2 _nextincrementdirection_2) (`self.AutoIncrementState` -1))
      (set `local.TmpState` _nextstateid_2)
      (set `local.TmpIncrementDirection` _nextincrementdirection_2))
    (:`NewEnumerator5`
      ;[1 1 1] Forces back to 0 state
      (set `local.TmpIncrementDirection` 1)
      (set `local.TmpState` 0))
    (:`NewEnumerator8`
      ;[1 1 1] Goes back to initial state
      (set `local.TmpIncrementDirection` 1)
      (set `local.TmpState` (`self.StartupStateId`))))
  (return (`local.TmpState`) (`local.TmpIncrementDirection`)))

(fn `ShouldFireChangedEvents`
  (params (NextStateId :type Byte) (PrevStateId :type Byte))
  (returns (bFireEvents :type Boolean))
  ;[1 1 1] Should fire success events if the new state is different than the old one, or, if we want to treat same state as a change state
  (return (or (!= NextStateId PrevStateId) (`self.bFireStateChangeOnSameState`))))

(fn `TryGetState`
  (params (StateId :type Byte))
  (returns (State :type String) (bValid :type Boolean))
  (bind _output (`|GetArrayItem` (`self.States`) (`KismetMathLibrary.Conv_ByteToInt` StateId)))
  (if (`self.IsStateIdValid` StateId)
    (return (select `bool` (== (`KismetStringLibrary.Len` _output) 0) :`false` _output :`true` (`KismetStringLibrary.Conv_ByteToString` StateId)) true)
    (else
      ;[1 1 1] State is not valid, return empty state
      (return "" false))))

(fn `UnBlockEvents`
  (set `self.bCanReceiveEvents` true))