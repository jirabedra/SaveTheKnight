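; Puzzle kit prototype for buttons and levers whose handle slides and/or rotates to show an IterativeStateComp state.
; The construction script builds an optional base mesh and slide/rotate joints beneath the handle.
; State changes queue sounds and timeline animations, with proportional, incremental or constant offsets; constant ones play back in reverse.
; The server replicates the state once the queue empties; clients delay handling it to avoid animation jitter.
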(event `self.ReceiveBeginPlay`
  ;[1 1 1] Set timeline animation speed
  (`TimelineComponent.SetPlayRate` (`self.ElementAnimation`) (/ 1.0 (`KismetMathLibrary.FMax` (`self.Duration`) 0.05)))
  ;[1 1 1] Try attach to handle
  (`self.PK_TryAttachChildren`)
  ;[1 1 1] Set Rotation relative to state
  (bind _output_get (set `self.NewStateId` (`.StateId` (`/Game/PuzzleKit-ButtonPrototype/Blueprints/Core/BP_PK_IterativeStateComponent.GetState` (`self.IterativeStateComp`)))))
  (bind _output_get_2 (set `self.PrevStateId` _output_get))
  (bind _output_get_3 (set `self.LastStateId` _output_get_2))
  (`self.ResetTransformToState` _output_get_3)
  (set `self.bIsPlayingAnimation` false))

(event `PlaySuccessEffects`
  (params (NewStateId :type Byte) (SuccessAction :type "/Game/PuzzleKit-ButtonPrototype/Blueprints/Core/Enums/EPK_StateAction Enum" :default "NewEnumerator9"))
  ;[0.5833 1 0.6334] On State Change Success play animation, sounds and trigger StateChanged
  (`KismetArrayLibrary.Array_Add` (`self.StateIdQueue`) (make `/Game/PuzzleKit-ButtonPrototype/Blueprints/Core/Structs/FPKAnimationQueueItem` NewStateId (select `/Game/PuzzleKit-ButtonPrototype/Blueprints/Core/Enums/EPK_StateAction` SuccessAction :`NewEnumerator9` true :`NewEnumerator3` true)))
  (if (not (`TimelineComponent.IsPlaying` (`self.ElementAnimation`)))
    (`self.PlayNextQueuedAnimation`)))

(event `self.PK_HandleOwnStateChanged`
  (params (NewStateId :type Byte) (Args :type "/Game/PuzzleKit-ButtonPrototype/Blueprints/Core/Structs/FPKStateChangeArgs Structure"))
  ;[0.5833 1 0.6334] On State Change Success play animation, sounds and trigger StateChanged
  (`self.PlaySuccessEffects` NewStateId Args_Reason_71_B758D633491B7A72BAA4FAAAD8C78C7E))

(event `PlayFailureEffects`
  ;[1 0.5573 0.5573] On State Change Failure only play sounds
  (`self.PlaySounds` (make `/Game/PuzzleKit-ButtonPrototype/Blueprints/Core/Structs/FPKAnimationQueueItem` (`self.LastStateId`))))

(event `self.PK_HandleOwnChangeFailure`
  (params (Args :type "/Game/PuzzleKit-ButtonPrototype/Blueprints/Core/Structs/FPKStateChangeArgs Structure") (FailReason :type "/Game/PuzzleKit-ButtonPrototype/Blueprints/Core/Enums/EPK_FailReason Enum" :default "NewEnumerator3"))
  ;[1 0.5573 0.5573] On State Change Failure only play sounds
  (`self.PlayFailureEffects`))

(event `PlayNextQueuedAnimation`
  (bind _output (`|GetArrayItem` (`self.StateIdQueue`)))
  ;[1 1 1] Play success efects from queue
  (if (> (`KismetArrayLibrary.Array_Length` (`self.StateIdQueue`)) 0)
    (`self.PlaySounds` _output)
    (`self.AnimateHandle` _output)
    (`KismetArrayLibrary.Array_Remove` (`self.StateIdQueue`))
    (else
      ;;[0.1473 0.6403 1] Replicate state when all animations from the queue finished playing.
      (`/Engine/EditorBlueprintResources/ActorMacros.Switch Has Authority`
        (:`Authority`
          (set `self.LastStateId` (`self.NewStateId`)))))))

(event `PlaySounds`
  (params (Animation :type "/Game/PuzzleKit-ButtonPrototype/Blueprints/Core/Structs/FPKAnimationQueueItem Structure"))
  ;[1 1 1] Play state transition sound
  (if (`self.bPlayTransitionSounds`)
    (if (`self.bUseStateDelta`)
      (`/Engine/EditorBlueprintResources/StandardMacros.CompareInt` (`KismetMathLibrary.Conv_ByteToInt` (`self.LastStateId`)) (`KismetMathLibrary.Conv_ByteToInt` Animation_StateId_4_47EEB643460777FBACA09C8FBB4D062A)
        (:`>`
          (`GameplayStatics.PlaySoundAtLocation` (`self.DownSound`) (`self.K2_GetActorLocation`) (struct) 1.0 1.0 0.0 null null null :!label _label))
        (:`==`
          (`GameplayStatics.PlaySoundAtLocation` (`self.NoChangeSound`) (`self.K2_GetActorLocation`) (struct) 1.0 1.0 0.0 null null null))
        (:`<`
          (`GameplayStatics.PlaySoundAtLocation` (`self.UpSound`) (`self.K2_GetActorLocation`) (struct) 1.0 1.0 0.0 null null null :!label _label_2)))
      (elif Animation_bIsForwardAnimation_7_605FD2454E79B56D498721977820BEEA
        (goto _label_2)
        (else
          (goto _label))))))

(event `AnimateHandle`
  (params (AnimItem :type "/Game/PuzzleKit-ButtonPrototype/Blueprints/Core/Structs/FPKAnimationQueueItem Structure"))
  ;[1 1 1] Animate Lever when State Changes
  (set `self.bIsPlayingAnimation` true)
  (set `self.NewStateId` AnimItem_StateId_4_47EEB643460777FBACA09C8FBB4D062A)
  (`|ExecutionSequence`
    (:`then_0`
      ;;[0.491 0.2918 0] Slide
      (bind _progress (`self.GetStateAnimationOffset` (`self.NewStateId`) (`self.PrevStateId`) (`self.PositionDeltaIs`) true AnimItem_bIsForwardAnimation_7_605FD2454E79B56D498721977820BEEA))
      (set `self.SlideAmount` _progress)
      ;;[0.1359 0.1426 0.2831] Rotation
      (bind _progress_2 (`self.GetStateAnimationOffset` (`self.NewStateId`) (`self.PrevStateId`) (`self.RotationAmplitudeIs`) true AnimItem_bIsForwardAnimation_7_605FD2454E79B56D498721977820BEEA))
      (set `self.RotationAmount` _progress_2))
    (:`then_1`
      (bind (_direction _alpha) (`Timeline|ElementAnimation` :!via `PlayFromStart` :!label _label_3)
        (:`Update`
          (`self.MoveLerp` (`self.SlideAmount`) _alpha)
          (`self.RotateLerp` (`self.RotationAmount`) _alpha))
        (:`Finished`
          (if (`self.ShouldReverseAnimation`)
            (`/Engine/EditorBlueprintResources/StandardMacros.FlipFlop` ; If is constant behaviour, we want to reverse once the effect and then continue
              (:`A`
                (goto _label_3 :!via `ReverseFromEnd`))
              (:`B`
                _)))
          ;;[1 1 1] Reset animation related variables
          (set `self.LastSlideOffset` (0.0 0.0 0.0))
          (set `self.LastRotation` (struct))
          (set `self.bIsPlayingAnimation` false)
          (set `self.PrevStateId` (`self.NewStateId`))
          (`self.PlayNextQueuedAnimation`))))))

(event `OnStateReplicated`
  ;[0.1473 0.6403 1] Called by OnRep_LastState
  ;;[1 1 1] QuickFix: animation jitter on clients, because of propagation delay
  (`KismetSystemLibrary.RetriggerableDelay` 0.5 :!label _label_4)
  (`/Game/PuzzleKit-ButtonPrototype/Blueprints/Core/BP_PK_IterativeStateComponent.UnBlockEvents` (`self.IterativeStateComp`))
  ;;[1 1 1] Only update transform if states are out of sync.
  (if (not (!= (`self.LastStateId`) (`self.NewStateId`)))
    ;;[1 1 1] Stop any playing animation
    (if (`self.bIsPlayingAnimation`)
      (goto _label_4)
      (else
        (`self.ResetTransformToState` (`self.LastStateId`))))))

(fn `GetStateAnimationOffset`
  (params (CurrentStateId :type Byte) (PreviousStateId :type Byte) (AnimationType :type "/Game/PuzzleKit-ButtonPrototype/Blueprints/Core/Enums/EPK_MovementOffsetType Enum" :default "NewEnumerator1") (bIsDuringAnimation :type Boolean) (bForward :type Boolean :default true))
  (returns (Progress :type "Float (double-precision)"))
  (locals (IdDelta :type "Float (double-precision)"))
  (set `local.IdDelta` (- (`KismetMathLibrary.Conv_ByteToDouble` CurrentStateId) (`KismetMathLibrary.Conv_ByteToDouble` PreviousStateId)))
  (return (select `/Game/PuzzleKit-ButtonPrototype/Blueprints/Core/Enums/EPK_MovementOffsetType` AnimationType :`NewEnumerator1` (/ (`local.IdDelta`) (`KismetMathLibrary.FMax` (`KismetMathLibrary.Conv_ByteToDouble` (`/Game/PuzzleKit-ButtonPrototype/Blueprints/Core/BP_PK_IterativeStateComponent.GetMaxStateId` (`self.IterativeStateComp`))) 1.0)) :`NewEnumerator0` (select `bool` bIsDuringAnimation :`true` 1.0 :!type "Float (single-precision)") :`NewEnumerator4` (select `bool` bIsDuringAnimation :`true` (select `bool` bForward :`false` -1.0 :`true` 1.0 :!type "Float (single-precision)")) :`NewEnumerator3` (`local.IdDelta`))))

(fn `MoveLerp`
  (params (Amount :type "Float (double-precision)") (Alpha :type "Float (double-precision)"))
  (bind _returnvalue (`KismetMathLibrary.VLerp` (0.0 0.0 0.0) (* (`self.PositionDelta`) Amount) Alpha))
  ;[0.491 0.3372 0.05286] Movement Animation
  (bind _slidejointcomponent (`self.SlideJointComponent`)
    (:`then`
      (`SceneComponent.K2_AddLocalOffset` _slidejointcomponent (- _returnvalue (`self.LastSlideOffset`)) false false)
      (set `self.LastSlideOffset` _returnvalue))
    (:`else`)))

(fn `MoveTo`
  (params (Amount :type "Float (double-precision)"))
  (bind _slidejointcomponent (`self.SlideJointComponent`)
    (:`then`
      (`SceneComponent.K2_SetRelativeLocation` _slidejointcomponent (+ (* (`self.PositionDelta`) Amount) (`self.InitialPositionOffset`)) false false)
      (set `self.LastSlideOffset` (0.0 0.0 0.0)))
    (:`else`)))

(fn `OnRep_LastState`
  ;[0.1473 0.6403 1] Call event, as we need a small delay before handling htis change
  (`self.OnStateReplicated`))

(fn `PK_IsBusy`
  (returns (bIsBusy :type Boolean))
  (return (`self.bIsPlayingAnimation`)))

(fn `PK_TryAttachChildren`
  (locals (Attached :type "Array of Actor Object Reference"))
  ;[1 1 1] If Attah Children To Handle is enabled, try to add all attached actors in the hierarchy to the Handle Mash
  (`/Engine/EditorBlueprintResources/StandardMacros.IsValid` (`self.HandleMeshComp`)
    (:`Is Valid`
      (if (`self.bAttachChildrenToHandle`)
        (bind _output_get (set `local.Attached` (`self.GetAttachedActors`)))
        (for _array_element _output_get
          (`/Engine/EditorBlueprintResources/StandardMacros.IsValid` _array_element
            (:`Is Valid`
              (`self.K2_AttachToComponent` _array_element (`self.HandleMeshComp`) "None" "KeepWorld" "KeepWorld" "KeepWorld" true))))))))

(fn `ResetTransformToState`
  (params (State :type Byte))
  (bind _returnvalue (`KismetMathLibrary.Clamp` (`KismetMathLibrary.Conv_ByteToInt` State) 0 (`KismetMathLibrary.Conv_ByteToInt` (`/Game/PuzzleKit-ButtonPrototype/Blueprints/Core/BP_PK_IterativeStateComponent.GetMaxStateId` (`self.IterativeStateComp`)))))
  (`|ExecutionSequence`
    (:`then_0`
      ;[0.491 0.3372 0.05286] Set Position based on Initial State
      (bind _progress (`self.GetStateAnimationOffset` (`KismetMathLibrary.Conv_IntToByte` _returnvalue) 0 (`self.PositionDeltaIs`)))
      (`self.MoveTo` _progress))
    (:`then_1`
      ;[0.1845 0.2016 0.2831] Set Rotation based on Initial State
      (bind _progress_2 (`self.GetStateAnimationOffset` (`KismetMathLibrary.Conv_IntToByte` _returnvalue) 0 (`self.RotationAmplitudeIs`)))
      (`self.RotateTo` _progress_2))))

(fn `RotateLerp`
  (params (Amount :type "Float (double-precision)") (Alpha :type "Float (double-precision)"))
  (bind _returnvalue (`KismetMathLibrary.RLerp` (struct) (* (`self.AmplitudeRotator`) Amount) Alpha (`self.bUseShortestPath`)))
  ;[0.1845 0.2016 0.2831] Rotation Animation
  (bind _rotatejointcomponent (`self.RotateJointComponent`)
    (:`then`
      (`SceneComponent.K2_AddLocalRotation` _rotatejointcomponent (`KismetMathLibrary.ComposeRotators` _returnvalue (`KismetMathLibrary.NegateRotator` (`self.LastRotation`))) false false)
      (set `self.LastRotation` _returnvalue))
    (:`else`)))

(fn `RotateTo`
  (params (Amount :type "Float (double-precision)"))
  ;[1 1 1] Resets the RotationJoint to the exact position
  (bind _rotatejointcomponent (`self.RotateJointComponent`)
    (:`then`
      (`SceneComponent.K2_SetRelativeRotation` :`self` _rotatejointcomponent)
      (`SceneComponent.K2_AddLocalRotation` _rotatejointcomponent (`KismetMathLibrary.ComposeRotators` (`self.InitialOffsetRotator`) (* (`self.AmplitudeRotator`) Amount)) false false)
      (set `self.LastRotation` (struct)))
    (:`else`)))

(fn `ShouldReverseAnimation`
  (returns (Reverse :type Boolean))
  (return (or (and (`self.bCanSlide`) (or (`|EnumEquality` (`self.PositionDeltaIs`) "NewEnumerator0") (`|EnumEquality` (`self.PositionDeltaIs`) "NewEnumerator4"))) (and (`self.bCanRotate`) (or (`|EnumEquality` (`self.RotationAmplitudeIs`) "NewEnumerator0") (`|EnumEquality` (`self.RotationAmplitudeIs`) "NewEnumerator4"))))))

(fn `ToAxisRotator`
  (params (Angle :type "Float (double-precision)"))
  (returns (Rotator :type "Rotator Structure"))
  (return (select `/Game/PuzzleKit-ButtonPrototype/Blueprints/Core/Enums/EPK_RotationAxis` (`self.RotationAxis`) :`NewEnumerator0` (`KismetMathLibrary.MakeRotator` Angle) :`NewEnumerator1` (`KismetMathLibrary.MakeRotator` 0.0 Angle) :`NewEnumerator2` (`KismetMathLibrary.MakeRotator` 0.0 0.0 Angle) :!type "Rotator Structure")))

(fn `UserConstructionScript`
  (locals (Root :type "SceneComponent Object Reference") (LastParent :type "SceneComponent Object Reference"))
  (bind _bsnaptosocket (`self.bSnapToSocket`))
  (bind _devicemeshcomp (`self.DeviceMeshComp`))
  (bind _returnvalue (select `bool` _bsnaptosocket :`false` "KeepRelative" :`true` "SnapToTarget" :!type "EAttachmentRule Enum"))
  (`|ExecutionSequence`
    (:`then_0`
      (set `local.LastParent` (`self.DefaultSceneRoot`)))
    (:`then_1`
      ;[1 1 1] Create Base Component
      (bind _basemesh (`self.BaseMesh`)
        (:`then`
          (bind _returnvalue_2 (`AddComponent|NODE_AddStaticMeshComponent-5`))
          (bind _output_get (set `self.DeviceMeshComp` _returnvalue_2))
          (`StaticMeshComponent.SetStaticMesh` _output_get _basemesh)
          (set `local.LastParent` (`self.DeviceMeshComp`))
          (bind _overridematerial (`self.OverrideMaterial`)
            (:`then`
              (`PrimitiveComponent.SetMaterial` _devicemeshcomp 0 _overridematerial)
              (set `self.DefaultSceneRoot` _devicemeshcomp))
            (:`else`)))
        (:`else`)))
    (:`then_2`
      ;[1 0.9585 0.5781] Create Slide Component, if CanSlide is true
      (if (`self.bCanSlide`)
        (bind _returnvalue_3 (`AddComponent|NODE_AddSceneComponent-0` :`bManualAttachment` true))
        (bind _output_get_2 (set `self.SlideJointComponent` _returnvalue_3))
        (`SceneComponent.K2_AttachToComponent` _output_get_2 (`local.LastParent`) (`self.JointSocketName`) "SnapToTarget" "SnapToTarget" "KeepRelative" false)
        (set `local.LastParent` (`self.SlideJointComponent`))))
    (:`then_3`
      ;[0.1845 0.2016 0.2831] Create Rotate Joint Component, if Can Rotate is true
      (if (`self.bCanRotate`)
        (bind _returnvalue_4 (`AddComponent|NODE_AddSceneComponent-1` :`bManualAttachment` true))
        (bind _output_get_3 (set `self.RotateJointComponent` _returnvalue_4))
        (`SceneComponent.K2_AttachToComponent` _output_get_3 (`local.LastParent`) (`self.JointSocketName`) "SnapToTarget" "SnapToTarget" "KeepRelative" true)
        (bind _rotator (`self.ToAxisRotator` (`self.RotationAmplitude`)))
        (set `self.AmplitudeRotator` _rotator)
        (bind _rotator_2 (`self.ToAxisRotator` (`self.InitialRotationOffset`)))
        (set `self.InitialOffsetRotator` _rotator_2)
        (set `local.LastParent` (`self.RotateJointComponent`))))
    (:`then_4`
      ;[1 1 1] Create Handle Component
      (`SceneComponent.K2_AttachToComponent` (`self.HandleMeshComp`) (`local.LastParent`) (select `bool` _bsnaptosocket :`true` (`self.JointSocketName`)) _returnvalue _returnvalue _returnvalue false)
      (`StaticMeshComponent.SetStaticMesh` (`self.HandleMeshComp`) (`self.HandleMesh`))
      ;;[1 1 1] Overwrite Handle Material
      (bind _separatehandlematerial (`self.SeparateHandleMaterial`)
        (:`then`
          (`PrimitiveComponent.SetMaterial` (`self.HandleMeshComp`) 0 _separatehandlematerial))
        (:`else`
          (bind _overridematerial_2 (`self.OverrideMaterial`)
            (:`then`
              (`PrimitiveComponent.SetMaterial` (`self.HandleMeshComp`) 0 _overridematerial_2))
            (:`else`)))))
    (:`then_5`
      ;[1 1 1] Set Rotation relative to state
      (`self.ResetTransformToState` 0))))